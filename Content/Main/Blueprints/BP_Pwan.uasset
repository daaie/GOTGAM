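; BP_Pwan holds a character's stat levels and a pool of bonus points for spending on those stats.
; AddLevel raises an indexed StatsLevels entry when enough points remain and deducts the cost, while GetStatsLevel returns a level by index.
; DecreaseLevel lowers a nonzero level but also subtracts points instead of refunding them.
; The 1 key grants bonus points and prints the total, apparently for testing.
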(event `AddLevel`
  (params (`Index Number = Stats Number` :type Integer) (`Points Required` :type Integer))
  (bind _statslevels (`self.StatsLevels`))
  ;[1 1 1] 캐릭터 스탯 포인트 더하기
  (if (>= (`self.CharacterBonusPoints`) `Points Required`)
    (`KismetArrayLibrary.Array_Set` _statslevels `Index Number = Stats Number` (+ (`|GetArrayItem` _statslevels `Index Number = Stats Number`) 1))
    (set `self.CharacterBonusPoints` (- (`self.CharacterBonusPoints`) `Points Required`))
    (else
      (`KismetSystemLibrary.PrintString` "nob" true true (struct :`R` 1.0 :`G` 0.175463 :`A` 1.0)))))

(event `DecreaseLevel`
  (params (`Stat Index Number` :type Integer) (`Points Needed` :type Integer))
  (bind _output (`|GetArrayItem` (`self.StatsLevels`) `Stat Index Number`))
  ;[1 1 1] 캐릭터 스탯 포인트 빼기
  (if (== _output 0)
    (`KismetSystemLibrary.PrintString` "nob" true true (struct :`R` 1.0 :`G` 0.175463 :`A` 1.0))
    (else
      (`KismetArrayLibrary.Array_Set` (`self.StatsLevels`) `Stat Index Number` (- _output 1))
      (set `self.CharacterBonusPoints` (- (`self.CharacterBonusPoints`) `Points Needed`)))))

(event `Key|One`
  (params (Key :type "Key Structure"))
  ;[1 1 1] 스텟 포인트 제공
  (:`Pressed`
    (bind _output_get (set `self.CharacterBonusPoints` (+ (`self.CharacterBonusPoints`) 3)))
    (`KismetSystemLibrary.PrintString` (`KismetStringLibrary.Conv_IntToString` _output_get))))

(fn `GetStatsLevel`
  (params (`Index Number = Stat Number` :type Integer))
  (returns (Return :type Integer))
  (return (`|GetArrayItem` (`self.StatsLevels`) `Index Number = Stat Number`)))

(fn `UserConstructionScript`)