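; Battle actor spawner that creates an enemy AI pawn when SpawnEnemy is called.
; On authority only, it spawns the pawn at the SpawnVolume location with the Arrow's rotation, flags it valid, stores the reference and sets WayPoint.
; The Damage event is empty; data-printing and defense-reduced ApplyDamage logic remain as disconnected nodes that never run.
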(event `SpawnEnemy`
  (`|ExecutionSequence`
    (:`then_0`
      (`/Engine/EditorBlueprintResources/ActorMacros.Switch Has Authority`
        (:`Authority`
          (bind _returnvalue (`AIBlueprintHelperLibrary.SpawnAIFromClass` (`self.AI Pawn`) null (`SceneComponent.K2_GetComponentLocation` (`self.SpawnVolume`)) (`SceneComponent.K2_GetComponentRotation` (`self.Arrow`))))
          (set `self.IsVaild?` true)
          (set `self.ActorSpawner_ActorS` _returnvalue)
          (set `self.WayPoint` (`self.WayPoint`)))))))

(event `Damage`
  (params (DamageTarget :type "/Game/Blueprints/Battle/ActorSpawner Object Reference")))

(fn `UserConstructionScript`)