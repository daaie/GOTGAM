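; Battle map game mode that assigns player order on login, sets up combat participants and ends the battle session.
; BeginPlay parses travel options, rolls monster IDs, bubble-sorts pre-placed participants by mesh tags into player, pet and enemy order, then destroys surplus slots.
; Once every player submits a pet number, it starts combat on registered controllers.
; Tick pushes enemy action states to controllers and destroys the session after battle when at most one controller remains.
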(event `self.K2_PostLogin`
  (params (NewPlayer :type "PlayerController Object Reference"))
  (`/Engine/EditorBlueprintResources/StandardMacros.IncrementInt` (`self.PCOrder`)
    (:`  `
      (bind _asbp_battle_map_pc (cast `/Game/Blueprints/Battle/Core/BP_BattleMapPC` NewPlayer))
      (set `/Game/Blueprints/Battle/Core/BP_BattleMapPC.PCOrder` (`self.PCOrder`) _asbp_battle_map_pc)
      (`/Game/Blueprints/Battle/Core/BP_BattleMapPC.ShowStartWidget` _asbp_battle_map_pc))))

(event `self.ReceiveTick`
  (params (DeltaSeconds :type "Float (single-precision)"))
  ;[1 1 1] 적 커맨드 클라이언트에게 뿌려줌
  (`self.S2C_EnemyCmd`)
  (`self.DestroyBattleSession`))

(event `S2C_EnemyCmd`
  ;[1 1 1] 적 커맨드 클라이언트에게 뿌려줌
  (for _array_element (`self.EnemyArray_GM`)
    (for _index (range (`self.PCOrder`))
      (bind _asbp_battle_map_pc (cast `/Game/Blueprints/Battle/Core/BP_BattleMapPC` (`GameplayStatics.GetPlayerController` _index)))
      (`/Game/Blueprints/Battle/Core/BP_BattleMapPC.S2C_EnemyCmd` _asbp_battle_map_pc _array_element (`/Game/Blueprints/Battle/Core/BP_Participant.EnemyActionState` _array_element)))))

(event `DestroyBattleSession`
  ;[1 1 1] 파티원이 한명남았을경우 세션 파괴 및 리턴 필드
  (if (`self.IsBattleEnd`)
    (bind _outactors (`GameplayStatics.GetAllActorsOfClass` "/Game/Blueprints/Battle/Core/BP_BattleMapPC.BP_BattleMapPC_C"))
    (if (<= (`KismetArrayLibrary.Array_Length` _outactors) 1)
      (`KismetSystemLibrary.Delay` 3.0)
      (`self.Destroy`))))

(event `AddParticipant`
  (params (Participant :type "/Game/Blueprints/Battle/Core/BP_Participant Object Reference"))
  (`/Engine/EditorBlueprintResources/StandardMacros.IsValid` Participant
    (:`Is Valid`
      (`KismetArrayLibrary.Array_AddUnique` (`self.Participants_GM`) Participant)
      (if (== (`|GetArrayItem` (`ActorComponent.ComponentTags` (`Character.Mesh` Participant))) "Enemy")
        (`KismetArrayLibrary.Array_AddUnique` (`self.EnemyArray_GM`) Participant)))))

(event `AddPCs`
  (params (PCs :type "/Game/Blueprints/Battle/Core/BP_BattleMapPC Object Reference"))
  (`/Engine/EditorBlueprintResources/StandardMacros.IsValid` PCs
    (:`Is Valid`
      (`KismetArrayLibrary.Array_AddUnique` (`self.PCs`) PCs))))

(event `SetNumParty`
  (bind _optionsstring (`self.OptionsString`))
  ;[1 1 1] 인원수 결졍
  ;;[1 0 0.03349] 수지가 건드렸읍니다
  (set `self.NumParty` (`KismetStringLibrary.Conv_StringToInt` (`GameplayStatics.ParseOption` _optionsstring "PartyNumber")))
  (bind _output_get (set `self.MonsterLevel` (`KismetStringLibrary.Conv_StringToInt` (`GameplayStatics.ParseOption` _optionsstring "MonsterLevel"))))
  (set `self.PlayerNum` 2)
  (bind _output_get_2 (set `self.EnemyNum` (`KismetMathLibrary.RandomIntegerInRange` 2 2)))
  (bind _output_get_3 (set `self.UserID` (`GameplayStatics.ParseOption` _optionsstring "ParticipantID")))
  (set `self.ServerID` _output_get_3)
  (for _ (range _output_get_2)
    ;;[1 1 1] 몬스터가 다다른종류가 나오는거?ㅋㅋㅋ
    (`KismetArrayLibrary.Array_Add` (`self.RandomMonsterNumber`) (`KismetMathLibrary.RandomIntegerInRange` 1000 1007)))
  (set `self.MonsterNumber` (make `/Game/Blueprints/Field/SpawnMonsterInfo` _output_get _output_get_2 (`self.RandomMonsterNumber`))))

(event `self.ReceiveBeginPlay`
  ;[0.4725 0 1] 승주가 만든거
  (`self.SetNumParty`)
  (bind _outactors (`GameplayStatics.GetAllActorsOfClass` "/Game/Blueprints/Battle/Core/BP_Participant.BP_Participant_C"))
  (set `self.Participants_GM` _outactors)
  (`self.AllofClassSort`)
  (`self.EnemyBattleNumSpawn` (`self.EnemyNum`))
  (`self.PlayerBattleNumSpawn` (`self.PlayerNum`))
  (`self.PlayerNumRefresh` 1))

(event `EnemyBattleNumSpawn`
  (params (EnemyNum :type Integer))
  (bind _participants_gm (`self.Participants_GM`))
  ;[0.4725 0 1] 승주가 만든거
  (set `self.LoopInt` 0)
  (bind (_arrayindex _arrayelement) (`/Engine/EditorBlueprintResources/StandardMacros.ReverseForEachLoop` (`self.Participants_GM`))
    (:`LoopBody`
      (if (> (- 8 EnemyNum) (`self.LoopInt`))
        (`/Engine/EditorBlueprintResources/StandardMacros.IncrementInt` (`self.LoopInt`)
          (:`  `
            (`self.K2_DestroyActor` _arrayelement)
            (`KismetArrayLibrary.Array_Remove` _participants_gm (`KismetArrayLibrary.Array_Find` _participants_gm _arrayelement))))))))

(event `PlayerBattleNumSpawn`
  (params (PlayerNum :type Integer))
  ;[0.4725 0 1] 승주가 만든거
  (for _array_element (`self.Participants_GM`)
    (bind _output (`|GetArrayItem` (`ActorComponent.ComponentTags` (`Character.Mesh` _array_element))))
    (if (== _output "Enemy")
      _
      (elif (== _output "Player")
        (switch `int` PlayerNum
          (:`0`
            (`KismetSystemLibrary.PrintString` "Not searching Player!"))
          (:`1`
            (`self.PlayerDestroy` 2)
            (`self.PlayerDestroy` 3)
            (`self.PlayerDestroy` 4))
          (:`2`
            (`self.PlayerDestroy` 3)
            (`self.PlayerDestroy` 4))
          (:`3`
            (`self.PlayerDestroy` 4)))))))

(event `PlayerDestroy`
  (params (PlayerNum :type Integer))
  (bind _participants_gm (`self.Participants_GM`))
  ;[0.4725 0 1] 승주가 만든거
  (for _array_element (`self.Participants_GM`)
    (bind _componenttags (`ActorComponent.ComponentTags` (`Character.Mesh` _array_element)))
    (bind _output (`|GetArrayItem` _componenttags))
    (if (== _output "Enemy")
      _
      (elif (== _output "Player")
        (if (== (`KismetStringLibrary.Conv_StringToInt` (`KismetStringLibrary.Conv_NameToString` (`|GetArrayItem` _componenttags 2))) PlayerNum) :!label _label
          (`self.K2_DestroyActor` _array_element)
          (`KismetArrayLibrary.Array_Remove` _participants_gm (`KismetArrayLibrary.Array_Find` _participants_gm _array_element)))
        (elif (== _output "Pet")
          (goto _label))))))

(event `PlayerNumRefresh`
  (params (PlayerNum :type Integer))
  ;[0.4725 0 1] 승주가 만든거
  (for _array_element (`self.Participants_GM`)
    (bind _componenttags (`ActorComponent.ComponentTags` (`Character.Mesh` _array_element)))
    (bind _output (`|GetArrayItem` _componenttags))
    (if (== _output "Enemy")
      _
      (elif (== _output "Player")
        (`KismetArrayLibrary.Array_Set` _componenttags 1 (`KismetStringLibrary.Conv_StringToName` (`KismetStringLibrary.Conv_IntToString` PlayerNum)))
        (`/Engine/EditorBlueprintResources/StandardMacros.IncrementInt` PlayerNum)))))

(event `AllofClassSort`
  ;[0.4725 0 1] 승주가 만든거
  (set `self.LoopInt` 0)
  (`self.StackVarInit`)
  (while (`self.WhileBreak`)
    (set `self.Part_Tmp` (`|GetArrayItem` (`self.Participants_GM`) (`self.LoopInt`)))
    (if (`self.NextTurnEnemy`)
      (`self.Sort` 8 (`self.Part_Tmp`) 2 "Enemy")
      (elif (`self.NextTurnPet`)
        (`self.Sort` 4 (`self.Part_Tmp`) 1 "Pet")
        (else
          (`self.Sort` 4 (`self.Part_Tmp`) 0 "Player")))))
  (set `self.Participants_GM` (`self.Participants_Stack`)))

(event `Participant_Sort`
  (params (SortArray :type "Array of /Game/Blueprints/Battle/Core/BP_Participant Object Reference") (NewParam :type Integer))
  ;[0.4725 0 1] 승주가 만든거
  (for (_array_element _array_index) SortArray
    (bind _returnvalue (+ _array_index 1))
    (if (< _returnvalue NewParam)
      (if (> (`KismetStringLibrary.Conv_StringToInt` (`KismetStringLibrary.Conv_NameToString` (`|GetArrayItem` (`ActorComponent.ComponentTags` (`Character.Mesh` _array_element)) 2))) (`KismetStringLibrary.Conv_StringToInt` (`KismetStringLibrary.Conv_NameToString` (`|GetArrayItem` (`ActorComponent.ComponentTags` (`Character.Mesh` (`|GetArrayItem` SortArray _returnvalue))) 2))))
        (`KismetArrayLibrary.Array_Swap` SortArray _array_index _returnvalue)
        (set `self.SortInt` 0)
        (else
          (bind _result (`/Engine/EditorBlueprintResources/StandardMacros.IncrementInt` (`self.SortInt`))
            (:`  `
              (if (not (<= _result NewParam))
                (set `self.Participants_Sort` SortArray))))))))
  (if (<= (`self.SortInt`) NewParam)
    (`self.Participant_Sort` SortArray NewParam)))

(event `StackVarInit`
  ;[0.4725 0 1] 승주가 만든거
  (set `self.LoopInt` 0)
  (`KismetArrayLibrary.Array_Clear` (`self.Participants_Sort`))
  (`KismetArrayLibrary.Array_Clear` (`self.Participants_Sort1`)))

(event `Sort`
  (params (Num :type Integer) (bp_Part :type "/Game/Blueprints/Battle/Core/BP_Participant Object Reference") (Player_Pet_Enemy :type Integer) (Player_Pet_Enemy_name :type Name))
  (bind _participants_sort1 (`self.Participants_Sort1`))
  ;[0.4725 0 1] 승주가 만든거
  (if (== (`|GetArrayItem` (`ActorComponent.ComponentTags` (`Character.Mesh` bp_Part))) Player_Pet_Enemy_name)
    (`KismetArrayLibrary.Array_Add` _participants_sort1 bp_Part)
    (if (>= (`KismetArrayLibrary.Array_Length` _participants_sort1) Num)
      (`self.Participant_Sort` _participants_sort1 Num)
      (`KismetArrayLibrary.Array_Append` (`self.Participants_Stack`) (`self.Participants_Sort`))
      (`self.StackVarInit`)
      (set `self.SortInt` 0)
      (switch `int` Player_Pet_Enemy
        (:`0`
          (set `self.NextTurnPet` true))
        (:`1`
          (set `self.NextTurnEnemy` true))
        (:`2`
          (set `self.WhileBreak` false)))
      (else
        (`/Engine/EditorBlueprintResources/StandardMacros.IncrementInt` (`self.LoopInt`))))
    (else
      (`/Engine/EditorBlueprintResources/StandardMacros.IncrementInt` (`self.LoopInt`)))))

(event `S2A_SetUpMeshOrStatus`
  (params (PetNumber :type Integer))
  ;[1 0.04144 0.8026] 클라이언트에게 매쉬 전송
  (`/Engine/EditorBlueprintResources/StandardMacros.IncrementInt` (`self.MeshCount`)
    (:`  `
      (`KismetArrayLibrary.Array_Add` (`self.MeshElement`) PetNumber)
      (if (== (`self.PlayerNum`) (`self.MeshCount`))
        (`self.SpawnMonster`)
        (for (_array_element _array_index) (`self.PCs`)
          (`/Game/Blueprints/Battle/Core/BP_BattleMapPC.InitiateCombat` _array_element (`|GetArrayItem` (`self.MeshElement`) _array_index) (`self.Monster`) (`self.PlayerNum`)))))))

(event `SpawnMonster`
  ;[1 1 1] 몬스터 스폰했으면 하는 건데
  (set `self.Monster` (`.MonsterNumber_14_E9B8153B428E7BD1E5DE25B7417AD52E` (break `/Game/Blueprints/Field/SpawnMonsterInfo` (`self.MonsterNumber`)))))

(fn `UserConstructionScript`)