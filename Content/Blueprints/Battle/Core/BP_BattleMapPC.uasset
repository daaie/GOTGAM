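; Player controller for a turn-based battle map, where each player commands a character and pet.
; BeginPlay registers with BP_BattleMapGM and finds owned participants by mesh tags; Tick copies the participant list.
; Command widgets run player then pet, with cursor-trace clicks choosing targets sent through C2S events.
; It also toggles custom-depth post-process highlights, sets combat meshes, and relays game-mode actions, defense and escape states to participants.
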(event `ReceiveInput_PC`
  (bind _currentparticipant_pc (`self.CurrentParticipant_PC`))
  (bind _playeractionstate (`/Game/Blueprints/Battle/Core/BP_Participant.PlayerActionState` (`self.CurrentParticipant_PC`)))
  (bind _petactionstate (`/Game/Blueprints/Battle/Core/BP_Participant.PetActionState` (`self.CurrentParticipant_PC`)))
  ;[1 1 1] 타겟팅관련
  (if (and (`|EnumEquality` (`/Game/Blueprints/Battle/Core/BP_Participant.FinalPlayerAction` _currentparticipant_pc) "NewEnumerator0") (`|EnumEquality` (`/Game/Blueprints/Battle/Core/BP_Participant.FinalPetAction` _currentparticipant_pc) "NewEnumerator0"))
    (if (== (`/Game/Blueprints/Battle/Core/BP_Participant.Team` _currentparticipant_pc) (`self.ControlledTeam`))
      (`|ExecutionSequence`
        (:`then_0`
          (`self.CheckValidTargetUnderCursor_PC`)
          (if (`self.TargetSucceed`)
            (if (`ActorComponent.ComponentHasTag` (`Character.Mesh` (`self.CurrentParticipant_PC`)) "Player")
              (switch `/Game/Blueprints/Battle/Core/ActionState_Player` _playeractionstate
                (:`NewEnumerator1`
                  _)
                (:`NewEnumerator3`
                  _)
                (:`NewEnumerator2`
                  _)
                (:`NewEnumerator4`
                  _))
              (`self.C2S_PlayerFinalAction` (`self.CurrentParticipant_PC`) (`self.CheckValidTargetUnderCursor_Return`) _playeractionstate)
              (`self.PlayerWidgetRemove`)
              (else
                (switch `/Game/Blueprints/Battle/Core/ActionState_Pet` _petactionstate
                  (:`NewEnumerator1`
                    _)
                  (:`NewEnumerator2`
                    _)
                  (:`NewEnumerator3`
                    _))
                (`self.C2S_PetFinalAction` (`self.CurrentParticipant_PC`) (`self.CheckValidTargetUnderCursor_Return`) _petactionstate)
                (`self.PetWidgetRemove`)))))
        (:`then_1`
          (`self.RemoveHighlight`))))))

(event `Key|LeftMouseButton`
  (params (Key :type "Key Structure"))
  ;[1 1 1] 타겟팅관련
  ;;[1 1 1] 마우스로 눌러서 타겟팅
  ;;;[1 1 1] 입력을 현재 Participant에게 전달
  (:`Pressed`
    (`self.CurrentParticipant_PC`
      (:`then`
        (`self.ReceiveInput_PC`))
      (:`else`))))

(event `GetParticipantUnderCursor`
  (bind (_hitresult _returnvalue) (`self.GetHitResultUnderCursorByChannel` "TraceTypeQuery3"))
  ;[1 1 1] 타겟팅관련
  ;;[1 1 1] 마우스로 눌러서 타겟팅
  ;;;[1 1 1] 마우스 커서 위치 추적
  (set `self.TraceHitResult` _hitresult)
  (if _returnvalue
    ;;;[1 1 1] 참가자 추적 결과 반환
    (bind _asbp_participant (cast `/Game/Blueprints/Battle/Core/BP_Participant` (`.HitActor` (`GameplayStatics.BreakHitResult` (`self.TraceHitResult`))))
      (:`then`
        ;;;;[1 1 1] result
        (set `self.PartipantUnderCursor` true)
        (set `self.Participant` _asbp_participant))
      (:`CastFailed`
        (set `self.PartipantUnderCursor` false) ; error
        (set `self.Participant` null)))
    (else
      (set `self.PartipantUnderCursor` false) ; error
      (set `self.Participant` null))))

(event `CheckValidTargetUnderCursor_PC`
  ;[1 1 1] 타겟팅관련
  (`self.GetParticipantUnderCursor`)
  (if (`self.PartipantUnderCursor`)
    (if (!= (`self.Participant`) (`self.CurrentParticipant_PC`))
      ;;[1 0.0629 0.4422] 클릭시 이벤트 (수정 필요)
      (`KismetSystemLibrary.PrintString` "Select Participate") ; 참가자 클릭함(적/팀 모두 ㅇㅋ)
      (set `self.TargetSucceed` true)
      ;;[1 1 1] 누른애가 제대로 배열에 있고 내가 아니라면
      (if (and (>= (`KismetArrayLibrary.Array_Find` (`self.Participants_Copy`) (`self.Participant`)) 0) (!= (`self.Participant`) (`self.CurrentParticipant_PC`)))
        (set `self.CheckValidTargetUnderCursor_Return` (`self.Participant`))
        (else
          (`self.RemoveHighlight`)))
      (else
        (`KismetSystemLibrary.PrintString` "huh?" :!label _label) ; 허공 클릭함
        (set `self.TargetSucceed` false)))
    (else
      (goto _label))))

(event `self.ReceiveTick`
  (params (DeltaSeconds :type "Float (single-precision)"))
  ;[1 0 0.5736] Debug용 (명령 입력 확인)
  (bind _asbp_battle_map_gm (cast `/Game/Blueprints/Battle/Core/BP_BattleMapGM` (`GameplayStatics.GetGameMode`)))
  (set `self.Participants_Copy` (`/Game/Blueprints/Battle/Core/BP_BattleMapGM.Participants` _asbp_battle_map_gm)))

(event `C2S_PlayerFinalAction`
  (params (PC_Partici :type "/Game/Blueprints/Battle/Core/BP_Participant Object Reference") (Target :type "/Game/Blueprints/Battle/Core/BP_Participant Object Reference") (state :type "/Game/Blueprints/Battle/Core/ActionState_Player Enum" :default "NewEnumerator0"))
  ;[1 1 1] 타겟팅 명령 서버로 보내주기
  (set `/Game/Blueprints/Battle/Core/BP_Participant.PreselectTarget` Target PC_Partici)
  (set `/Game/Blueprints/Battle/Core/BP_Participant.FinalPlayerAction` state PC_Partici))

(event `C2S_PetFinalAction`
  (params (PC_Partici :type "/Game/Blueprints/Battle/Core/BP_Participant Object Reference") (Target :type "/Game/Blueprints/Battle/Core/BP_Participant Object Reference") (state :type "/Game/Blueprints/Battle/Core/ActionState_Pet Enum" :default "NewEnumerator0"))
  ;[1 1 1] 타겟팅 명령 서버로 보내주기
  (set `/Game/Blueprints/Battle/Core/BP_Participant.PreselectTarget` Target PC_Partici)
  (set `/Game/Blueprints/Battle/Core/BP_Participant.FinalPetAction` state PC_Partici))

(event `self.ReceiveBeginPlay`
  ;[1 1 1] 하이라이트 마테리얼 설정
  (bind _returnvalue (`KismetMaterialLibrary.CreateDynamicMaterialInstance` "/Game/Materials/M_BattleHighlight_Inst.M_BattleHighlight_Inst"))
  (bind _output_get (set `self.HighlightMaterial` _returnvalue))
  (`PostProcessComponent.AddOrUpdateBlendable` (`self.High`) _output_get 1.0)
  ;[1 1 1] 위젯 입력 허용 설정
  (`WidgetBlueprintLibrary.SetInputMode_GameAndUIEx` self)
  ;[1 1 1] 본인 저장
  (bind _gamemode (`self.GetGameMode`))
  (`KismetArrayLibrary.Array_AddUnique` (`/Game/Blueprints/Battle/Core/BP_BattleMapGM.PCs` _gamemode) self)
  (set `self.MyPC` (`KismetSystemLibrary.GetDisplayName` self))
  ;[1 1 1] 자기 소유 플레이어/펫 찾기
  (for (_array_element _array_index) (`self.MaxPlayer`)
    (if (`KismetStringLibrary.EqualEqual_StrStr` _array_element (`self.MyPC`))
      (`self.FindMyPlayerPet` (+ _array_index 1)))))

(event `FindMyPlayerPet`
  (params (Num :type Integer))
  ;[1 1 1] 자기 소유 플레이어/펫 저장
  (bind _gamemode (`self.GetGameMode`))
  (for _array_element (`/Game/Blueprints/Battle/Core/BP_BattleMapGM.Participants` _gamemode)
    (`|ExecutionSequence`
      (:`then_0`
        (bind _componenttags (`ActorComponent.ComponentTags` (`Character.Mesh` _array_element)))
        (bind _returnvalue (== (`|GetArrayItem` _componenttags 1) (`KismetStringLibrary.Conv_StringToName` (`KismetStringLibrary.Conv_IntToString` Num))))
        (if (and (== (`|GetArrayItem` _componenttags) "Player") _returnvalue)
          (set `self.OwningPlayer` _array_element)))
      (:`then_1`
        (if (and _returnvalue (== (`|GetArrayItem` _componenttags) "Pet"))
          (set `self.OwningPet` _array_element))))))

(event `MultiDivision_Player`
  (params (State :type "/Game/Blueprints/Battle/Core/ActionState_Player Enum" :default "NewEnumerator0"))
  (bind _owningplayer (`self.OwningPlayer`))
  ;[1 1 1] 각 명령 뿌려주기 (확 줄인 버전)
  (bind _output_get (set `/Game/Blueprints/Battle/Core/BP_Participant.PlayerActionState` State _owningplayer))
  (`/Game/Blueprints/Battle/Core/BP_Participant.SetPlayerActionState` _owningplayer _output_get self)
  (set `self.CurrentParticipant_PC` _owningplayer))

(event `MultiDivision_Pet`
  (params (State :type "/Game/Blueprints/Battle/Core/ActionState_Pet Enum" :default "NewEnumerator0"))
  (bind _owningpet (`self.OwningPet`))
  ;[1 1 1] 각 명령 뿌려주기 (확 줄인 버전)
  (bind _output_get (set `/Game/Blueprints/Battle/Core/BP_Participant.PetActionState` State _owningpet))
  (`/Game/Blueprints/Battle/Core/BP_Participant.SetPetActionState` _owningpet _output_get self)
  (set `self.CurrentParticipant_PC` _owningpet))

(event `PlayerWidgetRemove`
  ;[1 1 1] 플레이어 커맨드 위젯 삭제
  (`Widget.RemoveFromParent` (`self.PlayerCmdWidget`))
  ;[1 1 1] 펫 죽었는지 검사
  (bind _owningpet (`self.OwningPet`)
    (:`then`
      (if (not (== (`KismetArrayLibrary.Array_Find` (`self.Participants_Copy`) _owningpet) -1))
        ;[1 1 1] 플레이어 커맨드 선택한 후, 펫 위젯 show
        (if (not (`/Game/Blueprints/Battle/Core/BP_Participant.IsRunReady` _owningpet))
          (if (not (`/Game/Blueprints/Battle/Core/BP_Participant.PlayerisDEAD` _owningpet))
            (`self.ShowPetCmdWidget` _owningpet)
            (else
              (`self.C2S_PetAlone` _owningpet "NewEnumerator5" :!label _label_2)))
          (else
            (goto _label_2)))))
    (:`else`)))

(event `C2S_PetAlone`
  (params (Partici :type "/Game/Blueprints/Battle/Core/BP_Participant Object Reference") (state :type "/Game/Blueprints/Battle/Core/ActionState_Pet Enum" :default "NewEnumerator0"))
  (bind _output_get (set `/Game/Blueprints/Battle/Core/BP_Participant.PetActionState` state Partici))
  (`/Game/Blueprints/Battle/Core/BP_Participant.SetPetActionState` Partici _output_get self))

(event `PetWidgetRemove`
  ;[1 1 1] 펫 커맨드 위뎃 삭제
  (`Widget.RemoveFromParent` (`self.PetCmdWidget`)))

(event `ShowStartBattleWidget`
  (bind _returnvalue (`|CreateWidget` "/Game/UMG/Battle/UMG_BattleMApStart.UMG_BattleMapStart_C" null "Welcome to Battle Map"))
  (`UserWidget.AddToViewport` _returnvalue 0))

(event `ShowInfoTextWidget`
  (params (Text :type String))
  (bind _returnvalue (`|CreateWidget` "/Game/UMG/Battle/UMG_BattleInfoText.UMG_BattleInfoText_C" null Text))
  (`UserWidget.AddToViewport` _returnvalue 0))

(event `ShowPlayerCmdWidget`
  (params (OwningParticipent :type "/Game/Blueprints/Battle/Core/BP_Participant Object Reference"))
  (bind _returnvalue (`|CreateWidget` "/Game/UMG/Battle/UMG_PlayerBattleMenu.UMG_PlayerBattleMenu_C" null OwningParticipent))
  (bind _output_get (set `self.PlayerCmdWidget` _returnvalue))
  (`UserWidget.AddToViewport` _output_get 0))

(event `ShowPetCmdWidget`
  (params (OwningParticipant :type "/Game/Blueprints/Battle/Core/BP_Participant Object Reference"))
  (bind _returnvalue (`|CreateWidget` "/Game/UMG/Battle/UMG_PetBattleMenu.UMG_PetBattleMenu_C" null OwningParticipant))
  (bind _output_get (set `self.PetCmdWidget` _returnvalue))
  (`UserWidget.AddToViewport` _output_get 0))

(event `RemoveHighlight`
  (for _array_element (`self.Participants_Copy`)
    (`self.Highlight` false (struct) _array_element)))

(event `TargetingHighlight`
  (params (MyTeam :type Integer) (Participant :type "/Game/Blueprints/Battle/Core/BP_Participant Object Reference"))
  (set `self.MyTeam` MyTeam)
  (bind _output_get (set `self.SearchThisParticipant` Participant))
  (if (!= (`/Game/Blueprints/Battle/Core/BP_Participant.Team` _output_get) (`self.MyTeam`))
    (`self.Highlight` true (struct :`R` 1.0 :`G` 0.62971 :`A` 1.0) _output_get)))

(event `Highlight`
  (params (`On/off` :type Boolean) (Value :type "LinearColor Structure") (Participant :type "/Game/Blueprints/Battle/Core/BP_Participant Object Reference"))
  (`MaterialInstanceDynamic.SetVectorParameterValue` (`self.HighlightMaterial`) "Colour" Value)
  (`PrimitiveComponent.SetRenderCustomDepth` (`Character.Mesh` Participant) `On/off`))

(event `InitiateCombat`
  (params (Participant :type "/Game/Blueprints/Battle/Core/BP_Participant Object Reference"))
  (bind _mesh (`Character.Mesh` Participant))
  ;[1 0 0.1301] *******캐릭터 메시 결정 (테스트중, 서버 필요)******** //플레이어, 펫, 적 순
  (if (== (`/Game/Blueprints/Battle/Core/BP_Participant.Team` Participant) 0)
    (if (== (`|GetArrayItem` (`ActorComponent.ComponentTags` _mesh)) "Player")
      (`SkinnedMeshComponent.SetSkinnedAssetAndUpdate` _mesh "/Game/Characters/Chara_4Hero.Chara_4Hero" false)
      (else
        (`SkinnedMeshComponent.SetSkinnedAssetAndUpdate` _mesh "/Game/Monsters/Stonemonster/StoneMonster_A.StoneMonster_A" false)
        (`SkeletalMeshComponent.SetAnimationMode` _mesh "AnimationBlueprint")
        (`SkeletalMeshComponent.SetAnimInstanceClass` _mesh "/Game/Monsters/Stonemonster/BattleStoneMonster/ABP_Battle_StoneMonster.ABP_Battle_StoneMonster_C")))
    (else
      (if (>= (`KismetMathLibrary.RandomFloat`) 0.5)
        (`SkinnedMeshComponent.SetSkinnedAssetAndUpdate` _mesh "/Game/Monsters/Stonemonster/StoneMonster_A.StoneMonster_A" false)
        (else
          (`SkinnedMeshComponent.SetSkinnedAssetAndUpdate` _mesh "/Game/Monsters/Stonemonster/StoneMonster_A.StoneMonster_A" false)))
      (`SkeletalMeshComponent.SetAnimationMode` _mesh "AnimationBlueprint")
      (`SkeletalMeshComponent.SetAnimInstanceClass` _mesh "/Game/Monsters/Stonemonster/BattleStoneMonster/ABP_Battle_StoneMonster.ABP_Battle_StoneMonster_C"))))

(event `Run_FindSameTag`
  (params (Player :type "/Game/Blueprints/Battle/Core/BP_Participant Object Reference"))
  ;[1 1 1] 도망_같은 태그 찾아 도망준비상태 만들기
  (for _array_element (`self.Participants_Copy`)
    (if (== (`|GetArrayItem` (`ActorComponent.ComponentTags` (`Character.Mesh` _array_element)) 1) (`|GetArrayItem` (`ActorComponent.ComponentTags` (`Character.Mesh` Player)) 1))
      (set `/Game/Blueprints/Battle/Core/BP_Participant.IsRunReady` true _array_element))))

(event `Defense`
  (for _array_element (`self.Participants_Copy`)
    (`/Engine/EditorBlueprintResources/StandardMacros.IsValid` _array_element
      (:`Is Valid`
        (`|ExecutionSequence`
          (:`then_0`
            ;[1 1 1] 액션모드 시작시, 방어 효과 적용
            (if (`/Game/Blueprints/Battle/Core/BP_Participant.IsDefence` _array_element)
              (`/Game/Blueprints/Battle/Core/BP_Participant.DefenceEffectFunc` _array_element)))
          (:`then_1`
            ;[1 1 1] 액션모드 시작시, 도망 준비
            (if (`/Game/Blueprints/Battle/Core/BP_Participant.IsRunReady` _array_element)
              (`/Game/Blueprints/Battle/Core/BP_Participant.RunReadyMotion` _array_element))))))))

(event `DefenseEnd`
  ;[1 1 1] 방어상태 해제
  (for _array_element (`self.Participants_Copy`)
    (bind _depenceparticleref (`/Game/Blueprints/Battle/Core/BP_Participant.DepenceParticleRef` _array_element))
    (`/Engine/EditorBlueprintResources/StandardMacros.IsValid` _depenceparticleref
      (:`Is Valid`
        (`ActorComponent.K2_DestroyComponent` _depenceparticleref)
        (`/Game/Blueprints/Battle/Core/BP_Participant.EndDefence` _array_element)))))

(event `GmToPc_AIController`
  (params (Enemy :type "/Game/Blueprints/Battle/Core/BP_Participant Object Reference") (`IsDefense?` :type Boolean))
  (bind _participants_copy (`self.Participants_Copy`))
  (if (== (`|GetArrayItem` (`ActorComponent.ComponentTags` (`Character.Mesh` Enemy))) "Enemy")
    (set `/Game/Blueprints/Battle/Core/BP_Participant.IsDefence` `IsDefense?` (`|GetArrayItem` _participants_copy (`KismetArrayLibrary.Array_Find` _participants_copy Enemy)))))

(event `GmToPc_PlayerOrPet`
  (params (PlayerOrPet :type "/Game/Blueprints/Battle/Core/BP_Participant Object Reference") (PlayerAction :type "/Game/Blueprints/Battle/Core/ActionState_Player Enum" :default "NewEnumerator0") (PetAction :type "/Game/Blueprints/Battle/Core/ActionState_Pet Enum" :default "NewEnumerator0"))
  (bind _participants_copy (`self.Participants_Copy`))
  (bind _output (`|GetArrayItem` (`ActorComponent.ComponentTags` (`Character.Mesh` PlayerOrPet))))
  (bind _output_2 (`|GetArrayItem` _participants_copy (`KismetArrayLibrary.Array_Find` _participants_copy PlayerOrPet)))
  (if (!= _output "Enemy")
    (if (== _output "Player")
      (set `/Game/Blueprints/Battle/Core/BP_Participant.FinalPlayerAction` PlayerAction _output_2)
      (elif (== _output "Pet")
        (set `/Game/Blueprints/Battle/Core/BP_Participant.FinalPetAction` PetAction _output_2)))))

(event `GmToPc_PreselectedAction`
  (params (CurrentParticipant :type "/Game/Blueprints/Battle/Core/BP_Participant Object Reference"))
  (bind _participants_copy (`self.Participants_Copy`))
  (`/Game/Blueprints/Battle/Core/BP_Participant.PreselectedAction` (`|GetArrayItem` _participants_copy (`KismetArrayLibrary.Array_Find` _participants_copy CurrentParticipant))))

(fn `UserConstructionScript`)