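; BP_Participant is a turn-based battle combatant, serving as player, pet or enemy, that registers with BP_BattleMapPC on spawn.
; Player and pet commands highlight targets or report through the PlayerController's C2S calls, while enemy AI randomly picks attack, defend or low-health flee.
; On its turn, it checks victory, rerolls invalid targets and branches by mesh component tag.
; Action execution is a placeholder print and delay before notifying the controller.
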(event `self.ReceiveBeginPlay`
  (`KismetSystemLibrary.Delay` 0.5)
  ;[1 1 1] 참가자 등록(PC)
  (bind _asbp_battle_map_pc (cast `/Game/Blueprints/Battle/Core/BP_BattleMapPC` (`GameplayStatics.GetPlayerController` 0)))
  (`/Game/Blueprints/Battle/Core/BP_BattleMapPC.AddParticipant` _asbp_battle_map_pc self)
  (`/Game/Blueprints/Battle/Core/BP_BattleMapPC.AddParticipant_Server` _asbp_battle_map_pc self))

(event `SetPlayerActionState`
  (params (NewState :type "/Game/Blueprints/Battle/Core/ActionState_Player Enum" :default "NewEnumerator0") (PC :type "/Game/Blueprints/Battle/Core/BP_BattleMapPC Object Reference"))
  (bind _playerpc (`self.PlayerPC`))
  (bind _playerpc_2 (`self.PlayerPC`))
  (bind _playerpc_3 (`self.PlayerPC`))
  (set `self.PlayerPC` PC)
  (bind _output_get (set `self.PlayerActionState` NewState))
  (switch `/Game/Blueprints/Battle/Core/ActionState_Player` _output_get
    (:`NewEnumerator1`
      ;[1 1 1] 공격,포획,스킬 - 타겟팅
      (for _array_element (`/Game/Blueprints/Battle/Core/BP_BattleMapPC.Participants_PC` _playerpc) :!label _label
        (`/Game/Blueprints/Battle/Core/BP_BattleMapPC.TargetingHighlight` _playerpc (`self.Team`) _array_element)))
    (:`NewEnumerator3`
      ;[1 1 1] 방어
      (bind _output_get_2 (set `self.FinalPlayerAction` "NewEnumerator3"))
      (bind _output_get_3 (set `self.IsDefence` true))
      (`/Game/Blueprints/Battle/Core/BP_BattleMapPC.RemovePlayerCmdWidget` _playerpc_3)
      (`/Game/Blueprints/Battle/Core/BP_BattleMapPC.C2S_PlayerCmd` _playerpc_3 self _output_get_2)
      (`/Game/Blueprints/Battle/Core/BP_BattleMapPC.C2S_Defence` _playerpc_3 self _output_get_3))
    (:`NewEnumerator2`
      ;[1 1 1] 도망
      (bind _output_get_4 (set `self.FinalPlayerAction` "NewEnumerator2"))
      (bind _output_get_5 (set `self.IsRunReady` true))
      (`/Game/Blueprints/Battle/Core/BP_BattleMapPC.Run_FindSameTag` (`self.PlayerPC`) self)
      (`/Game/Blueprints/Battle/Core/BP_BattleMapPC.RemovePlayerCmdWidget` _playerpc_2)
      (`/Game/Blueprints/Battle/Core/BP_BattleMapPC.C2S_PlayerCmd` _playerpc_2 self _output_get_4)
      (`/Game/Blueprints/Battle/Core/BP_BattleMapPC.C2S_RunReady` _playerpc_2 self _output_get_5))
    (:`NewEnumerator4`
      (goto _label))))

(event `SetPetActionState`
  (params (NewState :type "/Game/Blueprints/Battle/Core/ActionState_Pet Enum" :default "NewEnumerator0") (PC :type "/Game/Blueprints/Battle/Core/BP_BattleMapPC Object Reference"))
  (bind _playerpc (`self.PlayerPC`))
  (set `self.PlayerPC` PC)
  (bind _output_get (set `self.PetActionState` NewState))
  (switch `/Game/Blueprints/Battle/Core/ActionState_Pet` _output_get
    (:`NewEnumerator1`
      (goto _label))
    (:`NewEnumerator2`
      ;[1 1 1] 방어
      (bind _output_get_2 (set `self.FinalPetAction` "NewEnumerator2"))
      (bind _output_get_3 (set `self.IsDefence` true))
      (`/Game/Blueprints/Battle/Core/BP_BattleMapPC.RemovePetCmdWidget` _playerpc)
      (`/Game/Blueprints/Battle/Core/BP_BattleMapPC.C2S_PetCmd` _playerpc self _output_get_2)
      (`/Game/Blueprints/Battle/Core/BP_BattleMapPC.C2S_Defence` _playerpc self _output_get_3))
    (:`NewEnumerator3`
      (goto _label))
    (:`NewEnumerator5`
      ;[1 1 1] 도망
      (bind _output_get_4 (set `self.FinalPetAction` "NewEnumerator5"))
      (`/Game/Blueprints/Battle/Core/BP_BattleMapPC.C2S_PetCmd` (`self.PlayerPC`) self _output_get_4))))

(event `AIControlledAction`
  (if (and (<= (/ (`self.Health`) (`self.MaxHealth`)) 0.2) (<= (`KismetMathLibrary.RandomFloat`) 0.5))
    (bind _output_get (set `self.EnemyActionState` "NewEnumerator2"))
    (`self.SetEnemyActionState` _output_get)
    (else
      (bind _output_get_2 (set `self.EnemyActionState` (select `bool` (`KismetMathLibrary.RandomBoolWithWeight` 0.7) :`false` "NewEnumerator3" :`true` "NewEnumerator1" :!type "/Game/Blueprints/Battle/Core/EnemyAI/ActionState_Enemy Enum")))
      (`self.SetEnemyActionState` _output_get_2))))

(event `SetEnemyActionState`
  (params (State :type "/Game/Blueprints/Battle/Core/EnemyAI/ActionState_Enemy Enum" :default "NewEnumerator0"))
  (bind _potentialtargets (`self.PotentialTargets`))
  (bind _output (`|GetArrayItem` _potentialtargets (`KismetMathLibrary.RandomIntegerInRange` 0 (`KismetArrayLibrary.Array_LastIndex` _potentialtargets))))
  (`KismetArrayLibrary.Array_Clear` (`self.PotentialTargets`))
  (bind _output_get (set `self.EnemyActionState` State))
  (switch `/Game/Blueprints/Battle/Core/EnemyAI/ActionState_Enemy` _output_get
    (:`NewEnumerator1`
      ;[1 1 1] 공격 - 타겟팅
      (bind _asbp_battle_map_gm (cast `/Game/Blueprints/Battle/Core/BP_BattleMapGM` (`GameplayStatics.GetGameMode`)))
      (for _array_element (`/Game/Blueprints/Battle/Core/BP_BattleMapGM.Participants_GM` _asbp_battle_map_gm)
        (if (!= (`/Game/Blueprints/Battle/Core/BP_Participant.Team` _array_element) (`self.Team`))
          (`KismetArrayLibrary.Array_AddUnique` (`self.PotentialTargets`) _array_element)))
      (`/Engine/EditorBlueprintResources/StandardMacros.IsValid` _output
        (:`Is Valid`
          (set `self.PreselectTarget` _output))))
    (:`NewEnumerator3`
      ;[1 1 1] 방어/도망
      (set `self.IsDefence` true))
    (:`NewEnumerator2`
      (set `self.IsRunReady` true))))

(event `DefenceEffect`
  ;[1 1 1] 방어 이펙트
  (bind _returnvalue (`GameplayStatics.SpawnEmitterAttached` "/Game/InfinityBladeEffects/Effects/FX_Mobile/ICE/combat/P_AOE_Ice_CircleAttack.P_AOE_Ice_CircleAttack" (`self.Mesh`) "None" (0.0 0.0 0.0) (struct) (0.5 0.5 0.5)))
  (set `self.DefenceEffectRef` _returnvalue))

(event `RunReadyMotion`
  (bind (_returnvalue_roll _returnvalue_pitch _returnvalue_yaw) (`KismetMathLibrary.BreakRotator` (`self.K2_GetActorRotation`)))
  ;[1 1 1] 도망 모션
  (`self.K2_SetActorRotation` (`KismetMathLibrary.MakeRotator` 0.0 0.0 (+ _returnvalue_yaw 180.0))))

(event `PreselectAction`
  ;[1 1 1] 루프방지 결과 나오면 False로 끝남
  (`self.CheckWon`)
  (if (not (`self.CheckWonVictory`))
    ;[1 1 1] 나 안죽었어?
    (if (not (`self.Dead`))
      (`self.CheckUsingTargeting`)
      (if (`self.CheckTargetingReturn`)
        ;[1 1 1] 타겟 안죽었고 안도망갔고 유효함?
        (if (and (not (`/Game/Blueprints/Battle/Core/BP_Participant.Dead` (`self.PreselectTarget`))) (not (`/Game/Blueprints/Battle/Core/BP_Participant.IsRun` (`self.PreselectTarget`))) (`KismetSystemLibrary.IsValid` (`self.PreselectTarget`)))
          (`self.ExecutePreselectedAction` :!label _label)
          (else
            (bind _asbp_battle_map_pc (cast `/Game/Blueprints/Battle/Core/BP_BattleMapPC` (`GameplayStatics.GetPlayerController` 0)))
            (set `self.CurrentParticipantsList` (`/Game/Blueprints/Battle/Core/BP_BattleMapPC.Participants_PC` _asbp_battle_map_pc))
            ;[1 1 1] 타겟이 죽거나 유효하지 않거나 같은팀이거나 도망갔으면 루프 돌림
            (while (or (`/Game/Blueprints/Battle/Core/BP_Participant.Dead` (`self.PreselectTarget`)) (`/Game/Blueprints/Battle/Core/BP_Participant.IsRun` (`self.PreselectTarget`)) (not (`KismetSystemLibrary.IsValid` (`self.PreselectTarget`))) (== (`/Game/Blueprints/Battle/Core/BP_Participant.Team` (`self.PreselectTarget`)) (`self.Team`)))
              ;[1 1 1] 랜덤으로 다른 타겟 고름
              (`self.GetRandomParticipant` (`self.CurrentParticipantsList`))
              (set `self.PreselectTarget` (`self.RandomParticipant`)))
            (`self.ExecutePreselectedAction`)))
        (else
          (goto _label)))
      (else
        (`self.EndAction`)))))

(event `CheckUsingTargeting`
  (bind _finalplayeraction (`self.FinalPlayerAction`))
  (bind _finalpetaction (`self.FinalPetAction`))
  ;[1 1 1] 타겟팅이 필요한 액션인지 확인
  (switch `name` (`|GetArrayItem` (`ActorComponent.ComponentTags` (`self.Mesh`)))
    (:`Player`
      (if (or (`|EnumEquality` _finalplayeraction "NewEnumerator1") (`|EnumEquality` _finalplayeraction "NewEnumerator4"))
        (set `self.CheckTargetingReturn` true :!label _label_2)
        (else
          (set `self.CheckTargetingReturn` false :!label _label_3))))
    (:`Pet`
      (if (or (`|EnumEquality` _finalpetaction "NewEnumerator1") (`|EnumEquality` _finalpetaction "NewEnumerator3"))
        (goto _label_2)
        (else
          (goto _label_3))))
    (:`Enemy`
      (if (`|EnumEquality` (`self.EnemyActionState`) "NewEnumerator1")
        (goto _label_2)
        (else
          (goto _label_3))))))

(event `GetRandomParticipant`
  (params (Participants :type "Array of /Game/Blueprints/Battle/Core/BP_Participant Object Reference"))
  ;[1 1 1] 랜덤 참가자 구하기
  (set `self.RandomParticipant` (`|GetArrayItem` Participants (`KismetMathLibrary.RandomIntegerInRange` 0 (`KismetArrayLibrary.Array_LastIndex` Participants)))))

(event `ExecutePreselectedAction`
  ;[1 1 1] 각 액션 시작
  (switch `name` (`|GetArrayItem` (`ActorComponent.ComponentTags` (`self.Mesh`)))
    (:`Player`
      (switch `/Game/Blueprints/Battle/Core/ActionState_Player` (`self.FinalPlayerAction`)
        (:`NewEnumerator0`
          (`self.EndAction` :!label _label_4))
        (:`NewEnumerator1`
          (`KismetSystemLibrary.PrintString` (`KismetStringLibrary.Concat_StrStr` (`KismetSystemLibrary.GetDisplayName` self) "Action") true true (struct :`G` 0.66 :`B` 1.0 :`A` 1.0) 22.0 :!label _label_5)
          (`KismetSystemLibrary.Delay` 0.5)
          (`self.EndAction`))
        (:`NewEnumerator3`
          (goto _label_5))))
    (:`Pet`
      (switch `/Game/Blueprints/Battle/Core/ActionState_Pet` (`self.FinalPetAction`)
        (:`NewEnumerator0`
          (goto _label_4))
        (:`NewEnumerator1`
          (goto _label_5))
        (:`NewEnumerator2`
          (goto _label_5))))
    (:`Enemy`
      (switch `/Game/Blueprints/Battle/Core/EnemyAI/ActionState_Enemy` (`self.EnemyActionState`)
        (:`NewEnumerator0`
          (goto _label_4))
        (:`NewEnumerator1`
          (goto _label_5))
        (:`NewEnumerator3`
          (goto _label_5))))))

(event `EndAction`
  ;[1 1 1] End Action
  (set `self.PlayerActionState` "NewEnumerator0")
  (set `self.PetActionState` "NewEnumerator0")
  (set `self.FinalPlayerAction` "NewEnumerator0")
  (set `self.FinalPetAction` "NewEnumerator0")
  (bind _asbp_battle_map_pc (cast `/Game/Blueprints/Battle/Core/BP_BattleMapPC` (`GameplayStatics.GetPlayerController` 0)))
  (`/Game/Blueprints/Battle/Core/BP_BattleMapPC.ParticipantEndAction` _asbp_battle_map_pc self))

(event `TimeRateRandomTarget`
  (params (PC :type "/Game/Blueprints/Battle/Core/BP_BattleMapPC Object Reference"))
  (bind _preselecttarget (`self.PreselectTarget`))
  ;[0.3098 0 1] 타이머 _ 랜덤 타겟
  (bind _asbp_battle_map_pc (cast `/Game/Blueprints/Battle/Core/BP_BattleMapPC` (`GameplayStatics.GetPlayerController` 0)))
  ;;[1 1 1] 타겟이 죽거나 유효하지 않거나 같은팀이거나 도망갔으면 루프 돌림
  (set `self.CurrentParticipantsList` (`/Game/Blueprints/Battle/Core/BP_BattleMapPC.Participants_PC` _asbp_battle_map_pc))
  (`/Engine/EditorBlueprintResources/StandardMacros.IsValid` _preselecttarget
    (:`Is Valid`
      (while (or (`/Game/Blueprints/Battle/Core/BP_Participant.Dead` _preselecttarget) (`/Game/Blueprints/Battle/Core/BP_Participant.IsRun` (`self.PreselectTarget`)) (not (`KismetSystemLibrary.IsValid` (`self.PreselectTarget`))) (== (`/Game/Blueprints/Battle/Core/BP_Participant.Team` (`self.PreselectTarget`)) (`self.Team`)))
        ;;[1 1 1] 랜덤으로 다른 타겟 고름
        (`self.GetRandomParticipant` (`self.CurrentParticipantsList`) :!label _label_6)
        (bind _output_get (set `self.PreselectTarget` (`self.RandomParticipant`)))
        (`/Game/Blueprints/Battle/Core/BP_BattleMapPC.C2S_Target` PC self _output_get)))
    (:`Is Not Valid`
      (goto _label_6))))

(event `CheckWon`
  (bind _currentparticipant (`self.CurrentParticipant`))
  ;[1 1 1] 참가자 탐색
  (bind _asbp_battle_map_pc (cast `/Game/Blueprints/Battle/Core/BP_BattleMapPC` (`GameplayStatics.GetPlayerController` 0)))
  (for _array_element (`/Game/Blueprints/Battle/Core/BP_BattleMapPC.Participants_PC` _asbp_battle_map_pc)
    (set `self.CurrentParticipant` _array_element)
    ;[1 1 1] 팀이 다 안죽었으면 아직 안죽었다고 반환
    (if (and (not (`/Game/Blueprints/Battle/Core/BP_Participant.Dead` _currentparticipant)) (!= (`/Game/Blueprints/Battle/Core/BP_Participant.Team` _currentparticipant) (`self.Team`)))
      (set `self.NotAllDead` true)))
  ;[1 1 1] 모든 팀 구성원이 죽었으면 true를 반환함
  (set `self.CheckWonVictory` (not (`self.NotAllDead`))))

(fn `UserConstructionScript`)