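; Battle spawner Blueprint that creates an AI-controlled pet pawn when its SpawnPet event is called.
; SpawnAIFromClass spawns the configured PetPawn class at the SpawnVolume's world location, facing along the Arrow component.
; The event then sets a validity flag, stores the spawned pawn as PetSpawnerPet and assigns the WayPoint.
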(event `SpawnPet`
  (`|ExecutionSequence`
    (:`then_0`
      (bind _returnvalue (`AIBlueprintHelperLibrary.SpawnAIFromClass` (`self.Pet Pawn`) null (`SceneComponent.K2_GetComponentLocation` (`self.SpawnVolume`)) (`SceneComponent.K2_GetComponentRotation` (`self.Arrow`))))
      (set `self.IsVaild?` true)
      (set `self.PetSpawner_Pet` _returnvalue)
      (set `self.WayPoint` (`self.WayPoint`)))))

(fn `UserConstructionScript`)