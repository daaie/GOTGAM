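; Battle player state (by its name) that syncs the player's character stats with a web server via form-encoded POST requests.
; On BeginPlay it takes the URL from the game instance and the battle player controller, then loads stats from JSON into Stat.
; UpdateBattle derives level-ups, state points and exp from a level×15 threshold, then posts them.
; Any non-empty item is sent as a hardcoded ID; the update response is ignored.
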(event `self.ReceiveBeginPlay`
  ;[1 1 1] 초기화
  (bind _asgame_instance (cast `/Game/Blueprints/AllLevels/GameInstance` (`GameplayStatics.GetGameInstance`)))
  (set `self.GameInstanceRef` _asgame_instance)
  (set `self.URL` (`/Game/Blueprints/AllLevels/GameInstance.URL` (`self.GameInstanceRef`)))
  (bind _asbp_battle_map_pc (cast `/Game/Blueprints/Battle/Core/BP_BattleMapPC` (`GameplayStatics.GetPlayerController` 0)))
  (set `self.BattlePCRef` _asbp_battle_map_pc)
  (`self.SelectCharacterStatus`))

(event `SelectCharacterStatus`
  ;[1 1 1] SelectCharacter
  (bind _output_get (set `self.Request` (`VaRestRequestJSON.ConstructRequestExt` "POST" "x_www_form_urlencoded_body")))
  (bind _returnvalue (`VaRestRequestJSON.GetRequestObject` _output_get))
  (set `self.RequestObject` _returnvalue)
  (`VaRestJsonObject.SetStringField` (`self.RequestObject`) "userid" (`/Game/Blueprints/Battle/Core/BP_BattleMapPC.UserID` (`self.BattlePCRef`)))
  (add `VaRestRequestJSON.OnRequestComplete` (`self.Request`) (delegate `SelectCharacterInfo`))
  (`VaRestRequestJSON.ProcessURL` (`self.Request`) (`KismetStringLibrary.Concat_StrStr` (`self.URL`) "/SelectCharacterStatus")))

(event `SelectCharacterInfo`
  (params (Request :type "VaRestRequestJSON Object Reference"))
  (bind _json (`self.Json`))
  ;[1 1 1] SelectCharacter
  (bind _returnvalue (`VaRestRequestJSON.GetResponseObject` Request))
  (set `self.Json` _returnvalue)
  (if (`VaRestJsonObject.GetBoolField` (`self.Json`) "Success")
    (set `self.Stat` (make `/Game/Blueprints/AllLevels/CharacterStat` (`VaRestJsonObject.GetStringField` _json "NickName") (`KismetStringLibrary.Conv_StringToInt` (`VaRestJsonObject.GetStringField` _json "Level")) (`KismetStringLibrary.Conv_StringToDouble` (`VaRestJsonObject.GetStringField` _json "Vital")) (`KismetStringLibrary.Conv_StringToDouble` (`VaRestJsonObject.GetStringField` _json "Exp")) (`KismetStringLibrary.Conv_StringToDouble` (`VaRestJsonObject.GetStringField` _json "Str")) (`KismetStringLibrary.Conv_StringToDouble` (`VaRestJsonObject.GetStringField` _json "Tgh")) (`KismetStringLibrary.Conv_StringToDouble` (`VaRestJsonObject.GetStringField` _json "Dex")) 0 0 0 0 0 "" (`KismetStringLibrary.Conv_StringToInt` (`VaRestJsonObject.GetStringField` _json "CurrentVital")) (`KismetStringLibrary.Conv_StringToInt` (`VaRestJsonObject.GetStringField` _json "StatePnt"))))
    (else
      (`KismetSystemLibrary.PrintString` "캐릭터 정보 로딩실패"))))

(event `UpdateBattle`
  (params (Exp :type Integer) (Item :type String))
  (bind _requestobject (`self.RequestObject`))
  (bind (_name _level _vital _exp _str _tgh _dex _attr _stamina _power _health _elabo _gender _currentvital _statepoint) (break `/Game/Blueprints/AllLevels/CharacterStat` (`self.Stat`)))
  (bind _returnvalue (+ (`KismetMathLibrary.Conv_IntToDouble` Exp) _exp))
  (bind _returnvalue_2 (* _level 15))
  (bind _returnvalue_3 (`KismetMathLibrary.FTrunc` (/ _returnvalue (`KismetMathLibrary.Conv_IntToDouble` _returnvalue_2))))
  ;[1 1 1] /UpdateBattleResults
  (bind _output_get (set `self.Request` (`VaRestRequestJSON.ConstructRequestExt` "POST" "x_www_form_urlencoded_body")))
  (bind _returnvalue_4 (`VaRestRequestJSON.GetRequestObject` _output_get))
  (set `self.RequestObject` _returnvalue_4)
  (bind _structout (setmembers `/Game/Blueprints/AllLevels/CharacterStat` :`StructRef` (`self.Stat`) :`Level` (+ _returnvalue_3 _level) :`Exp` (+ _exp (`KismetMathLibrary.Conv_IntToDouble` (mod (`KismetMathLibrary.FTrunc` _returnvalue) _returnvalue_2))) :`StatePoint` (+ _statepoint _returnvalue_3)))
  (`VaRestJsonObject.SetStringField` _requestobject "userid" (`/Game/Blueprints/Battle/Core/BP_BattleMapPC.UserID` (`self.BattlePCRef`)))
  (bind (_name_2 _level_2 _vital_2 _exp_2 _str_2 _tgh_2 _dex_2 _attr_2 _stamina_2 _power_2 _health_2 _elabo_2 _gender_2 _currentvital_2 _statepoint_2) (break `/Game/Blueprints/AllLevels/CharacterStat` _structout))
  (`VaRestJsonObject.SetNumberField` _requestobject "exp" _exp_2)
  (`VaRestJsonObject.SetIntegerField` _requestobject "level" _level_2)
  (`VaRestJsonObject.SetIntegerField` _requestobject "statePnt" _statepoint_2)
  (if (not (`KismetStringLibrary.EqualEqual_StrStr` Item))
    (`VaRestJsonObject.SetIntegerField` _requestobject "item" 6))
  (add `VaRestRequestJSON.OnRequestComplete` (`self.Request`) (delegate `UpdateBattleResults`))
  (`VaRestRequestJSON.ProcessURL` (`self.Request`) (`KismetStringLibrary.Concat_StrStr` (`self.URL`) "/UpdateBattleResults")))

(event `UpdateBattleResults`
  (params (Request :type "VaRestRequestJSON Object Reference"))
  ;[1 1 1] /UpdateBattleResults
)

(fn `UserConstructionScript`)