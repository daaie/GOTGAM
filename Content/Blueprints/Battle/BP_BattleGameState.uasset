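; Battle game state that fetches a player's battle pet from a web backend and stores it in the party pet list.
; SelectMyPet sends the BattlePC's user ID in a form-encoded POST request to the SelectBattlePet endpoint.
; The completion callback reads the JSON response, builds a pet status from its identity, level, stats, status and skill fields, and appends it to PartyPetStatus.
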(event `SelectMyPet`
  (params (BattlePC :type "/Game/Blueprints/Battle/Core/BP_BattleMapPC Object Reference"))
  ;[1 1 1] SelectPet
  (bind _output_get (set `self.Request` (`VaRestRequestJSON.ConstructRequestExt` "POST" "x_www_form_urlencoded_body")))
  (bind _returnvalue (`VaRestRequestJSON.GetRequestObject` _output_get))
  (set `self.RequestObject` _returnvalue)
  (`VaRestJsonObject.SetStringField` (`self.RequestObject`) "userid" (`/Game/Blueprints/Battle/Core/BP_BattleMapPC.UserID` BattlePC))
  (add `VaRestRequestJSON.OnRequestComplete` (`self.Request`) (delegate `CustomEvent`))
  (`VaRestRequestJSON.ProcessURL` (`self.Request`) (`KismetStringLibrary.Concat_StrStr` (`self.URL`) "/SelectBattlePet")))

(event `CustomEvent`
  (params (Request :type "VaRestRequestJSON Object Reference"))
  (bind _jsonpet (`self.JsonPet`))
  ;[1 1 1] SelectPet
  (bind _returnvalue (`VaRestRequestJSON.GetResponseObject` Request))
  (bind _output_get (set `self.JsonPet` _returnvalue))
  (`/Engine/EditorBlueprintResources/StandardMacros.IsValid` _output_get
    (:`Is Valid`
      (bind _output_get_2 (set `self.PetStatus` (make `/Game/Blueprints/AllLevels/PetStat` (`VaRestJsonObject.GetIntegerField` _jsonpet "pet_id") (`VaRestJsonObject.GetStringField` _jsonpet "pet_name") (`VaRestJsonObject.GetIntegerField` _jsonpet "level") (`VaRestJsonObject.GetNumberField` _jsonpet "exp") (`VaRestJsonObject.GetNumberField` _jsonpet "current_vital") (`VaRestJsonObject.GetNumberField` _jsonpet "vital") (`VaRestJsonObject.GetNumberField` _jsonpet "str") (`VaRestJsonObject.GetNumberField` _jsonpet "tgh") (`VaRestJsonObject.GetNumberField` _jsonpet "dex") (`VaRestJsonObject.GetStringField` _jsonpet "status") (`VaRestJsonObject.GetStringField` _jsonpet "pet_skill"))))
      (`KismetArrayLibrary.Array_Add` (`self.PartyPetStatus`) _output_get_2))))

(fn `UserConstructionScript`)