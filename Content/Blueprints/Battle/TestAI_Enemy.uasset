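; Test enemy character for a turn-based battle that can be hovered or clicked as a target and picks its own action.
; Hover and click swap the body material; a click also stores its location and disables player mouse events for three seconds.
; Tick switches on state, randomly choosing attack (weighted) or defence outside Wait.
; Action events write state and turn-over flags to the enemy AI controller's Blackboard; damage is only printed.
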(event `self.ReceiveBeginPlay`
  ;[1 1 1] 원래 마테리얼 저장
  (set `self.OriginMaterial` (`PrimitiveComponent.GetMaterial` (`self.Body`) 0)))

(event `self.ReceiveTick`
  (params (DeltaSeconds :type "Float (single-precision)"))
  (bind _returnvalue (`GameplayStatics.GetPlayerController` 0))
  (bind _returnvalue_2 (`GameplayStatics.GetPlayerController` 0))
  (`|ExecutionSequence`
    (:`then_0`
      (`|ExecutionSequence`
        (:`then_0`
          (if (`self.IsClicked`)
            (set `PlayerController.bEnableMouseOverEvents` false _returnvalue)
            (set `PlayerController.bEnableClickEvents` false _returnvalue)
            (`KismetSystemLibrary.Delay` 3.0) ; 딜레이 후, 원상태로 돌아옴
            (set `PlayerController.bEnableMouseOverEvents` true _returnvalue_2)
            (set `PlayerController.bEnableClickEvents` true _returnvalue_2)
            (set `self.IsClicked` false)))))
    (:`then_1`
      ;[1 1 1] 적 스위치
      (switch `/Game/Blueprints/AI/EnemyState` (`self.StateBP`)
        (:`NewEnumerator3`
          (`self.On_Wait`))
        (:`NewEnumerator0`
          (if (`KismetMathLibrary.RandomBoolWithWeight` 0.7) :!label _label
            (`self.On_Attack`)
            (else
              (`self.On_Defence`))))
        (:`NewEnumerator1`
          (goto _label))))))

(event `self.CapsuleComponent.OnClicked`
  (params (TouchedComponent :type "PrimitiveComponent Object Reference") (ButtonPressed :type "Key Structure"))
  ;[1 1 1] 클릭
  (`PrimitiveComponent.SetMaterial` (`self.Body`) 0 (`self.ChangeMaterial`))
  (set `self.IsClicked` true)
  ;[1 1 1] 클릭된 오브제 위치 저장
  (bind _output_get (set `self.TargetLoc` (`self.K2_GetActorLocation`)))
  (`KismetSystemLibrary.PrintString` (`KismetStringLibrary.Conv_VectorToString` _output_get)))

(event `InitEnemyState`
  (`self.Set State` "NewEnumerator3")
  (`self.Set ActionOver` false))

(event `self.CapsuleComponent.OnBeginCursorOver`
  (params (TouchedComponent :type "PrimitiveComponent Object Reference"))
  ;[1 1 1] 커서 오버랩
  (`PrimitiveComponent.SetMaterial` (`self.Body`) 0 (`self.ChangeMaterial`)))

(event `Set State`
  (params (NewParam :type "/Game/Blueprints/AI/EnemyState Enum" :default "NewEnumerator3"))
  ;[1 1 1] 상태 저장
  (bind _output_get (set `self.StateBP` NewParam))
  (bind _asbp_enemy_controllor (cast `/Game/Blueprints/AI/BP_EnemyControllor` (`AIBlueprintHelperLibrary.GetAIController` self)))
  (`BlackboardComponent.SetValueAsEnum` (`AIBlueprintHelperLibrary.GetBlackboard` _asbp_enemy_controllor) "State" _output_get))

(event `self.ReceiveAnyDamage`
  (params (Damage :type "Float (single-precision)") (DamageType :type "DamageType Object Reference") (InstigatedBy :type "Controller Object Reference") (DamageCauser :type "Actor Object Reference"))
  ;[1 1 1] HPBarUpdate
  (`KismetSystemLibrary.PrintString` (`KismetStringLibrary.Conv_DoubleToString` (- 0.0 Damage))))

(event `self.CapsuleComponent.OnEndCursorOver`
  (params (TouchedComponent :type "PrimitiveComponent Object Reference"))
  ;[1 1 1] 커서 오버랩
  (if (not (`self.IsClicked`))
    (`PrimitiveComponent.SetMaterial` (`self.Body`) 0 (`self.OriginMaterial`))))

(event `On_Wait`
  ;[1 1 1] AI 상태
)

(event `On_Attack`
  ;[1 1 1] AI 상태
  (`self.Set State` "NewEnumerator0")
  (`self.Set ActionOver` true :!label _label_2))

(event `On_Defence`
  ;[1 1 1] AI 상태
  (`self.Set State` "NewEnumerator1")
  (goto _label_2))

(event `On_Escape`
  ;[1 1 1] AI 상태
  (`self.Set State` "NewEnumerator2")
  (goto _label_2))

(event `Set ActionOver`
  (params (NewParam :type Boolean))
  ;[1 1 1] 턴종료
  (bind _output_get (set `self.IsAcionOver?` NewParam))
  (bind _asbp_enemy_controllor (cast `/Game/Blueprints/AI/BP_EnemyControllor` (`AIBlueprintHelperLibrary.GetAIController` self)))
  (`BlackboardComponent.SetValueAsBool` (`AIBlueprintHelperLibrary.GetBlackboard` _asbp_enemy_controllor) "IsMyAcionOver?" _output_get))

(fn `UserConstructionScript`)