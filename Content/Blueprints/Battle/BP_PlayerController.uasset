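; Battle player controller that runs the attack, defend, capture and run actions for the party member at TestSlot in the game mode's PlayerS array, then advances the slot.
; Attack uses timelines to lerp that member toward TestAI_Enemy target locations and back; run lifts and destroys it.
; Defend and capture are placeholders that spawn an emitter and print.
; AddLevel spends CharacterPoints to raise a stat; DecreaseLevel and GetStatsLevel are empty.
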(event `testNext`
  ;[1 1 1] 테스트용: 다음 슬롯 지정
  (`/Engine/EditorBlueprintResources/StandardMacros.IncrementInt` (`self.testSlot`)))

(event `AttackActFunc`
  (bind _testslot (`self.testSlot`))
  ;[1 1 1] 1. 공격버튼
  (bind _asbp_first_person_game_mode (cast `/Game/Blueprints/FirstPersonBP/BP_FirstPersonGameMode` (`GameplayStatics.GetGameMode`)))
  (bind _players (`/Game/Blueprints/FirstPersonBP/BP_FirstPersonGameMode.PlayerS` _asbp_first_person_game_mode))
  (set `self.StartLocation` (`self.K2_GetActorLocation` (`|GetArrayItem` _players _testslot)))
  (bind (_direction _move) (`Timeline|타임라인_0` :!via `PlayFromStart`)
    (:`Update`
      (bind _outactors (`GameplayStatics.GetAllActorsOfClass` "/Game/Blueprints/Battle/TestAI_Enemy.TestAI_Enemy_C"))
      (for _array_element _outactors
        (bind _output (`|GetArrayItem` _players _testslot))
        (bind _rootcomponent (`Actor.RootComponent` _output))
        (`SceneComponent.K2_SetWorldLocation` _rootcomponent (`KismetMathLibrary.VLerp` (`self.StartLocation`) (`/Game/Blueprints/Battle/TestAI_Enemy.TargetLoc` _array_element) _move) true true)))
    (:`Finished`
      (bind (_direction_2 _move_2) (`Timeline|타임라인_1` :!via `PlayFromStart`)
        (:`Update`
          (`SceneComponent.K2_SetWorldLocation` _rootcomponent (`KismetMathLibrary.VLerp` (`self.K2_GetActorLocation` _output) (`self.StartLocation`) _move_2) false true))
        (:`Finished`
          (`self.testNext`))))))

(event `RunActFunc`
  (bind _testslot (`self.testSlot`))
  ;[1 1 1] 3. 도망버튼
  (bind _asbp_first_person_game_mode (cast `/Game/Blueprints/FirstPersonBP/BP_FirstPersonGameMode` (`GameplayStatics.GetGameMode`)))
  (bind (_direction _move) (`Timeline|타임라인_2` :!via `PlayFromStart`)
    (:`Update`
      (bind _output (`|GetArrayItem` (`/Game/Blueprints/FirstPersonBP/BP_FirstPersonGameMode.PlayerS` _asbp_first_person_game_mode) _testslot))
      (bind _returnvalue (`self.K2_GetActorLocation` _output))
      (`SceneComponent.K2_SetWorldLocation` (`Actor.RootComponent` _output) (`KismetMathLibrary.VLerp` _returnvalue (+ _returnvalue (0.0 0.0 100.0)) _move) true false))
    (:`Finished`
      (`self.K2_DestroyActor` _output)
      (`KismetSystemLibrary.PrintString` (`KismetStringLibrary.Concat_StrStr` "Player" (`KismetStringLibrary.Conv_IntToString` _testslot) ": Run Success!") true true (struct :`G` 0.66 :`B` 1.0 :`A` 1.0) 5.0)
      (`self.testNext`))))

(event `CaptureActFunc`
  ;[1 1 1] 4. 포획 버튼
  (bind _asbp_first_person_game_mode (cast `/Game/Blueprints/FirstPersonBP/BP_FirstPersonGameMode` (`GameplayStatics.GetGameMode`)))
  (`GameplayStatics.SpawnEmitterAtLocation` null (`self.K2_GetActorLocation` (`|GetArrayItem` (`/Game/Blueprints/FirstPersonBP/BP_FirstPersonGameMode.PlayerS` _asbp_first_person_game_mode) (`self.testSlot`))))
  (`KismetSystemLibrary.PrintString` "4. Capture Button is clicked")
  (`self.testNext`))

(event `DepenceActFunc`
  ;[1 1 1] 2. 방어버튼
  (bind _asbp_first_person_game_mode (cast `/Game/Blueprints/FirstPersonBP/BP_FirstPersonGameMode` (`GameplayStatics.GetGameMode`)))
  (`GameplayStatics.SpawnEmitterAtLocation` null (`self.K2_GetActorLocation` (`|GetArrayItem` (`/Game/Blueprints/FirstPersonBP/BP_FirstPersonGameMode.PlayerS` _asbp_first_person_game_mode) (`self.testSlot`))))
  (`KismetSystemLibrary.PrintString` "2. Depence Button is clicked")
  (`self.testNext`))

(event `AddLevel`
  (params (`Index Number = Stats Number` :type Integer) (`Points Required` :type Integer))
  (bind _statslevels (`self.StatsLevels`))
  (if (>= (`self.CharacterPoints`) `Points Required`)
    (`KismetArrayLibrary.Array_Set` _statslevels `Index Number = Stats Number` (+ (`|GetArrayItem` _statslevels `Index Number = Stats Number`) 1))
    (set `self.CharacterPoints` (- (`self.CharacterPoints`) `Points Required`))
    (else
      (`KismetSystemLibrary.PrintString` "nob" true true (struct :`R` 1.0 :`G` 0.175463 :`A` 1.0)))))

(event `DecreaseLevel`)

(event `GetStatsLevel`)

(fn `UserConstructionScript`)