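; Test Blueprint that rolls randomized enemy stats from a data table and prints them on BeginPlay.
; It reads row "1000" of EnemyDataTable and truncates base Vital, Str, Tgh and Dex into an array.
; PointStats adds a random share of the shrinking RandomPoint pool to each stat in order, possibly leaving points unspent.
; BonusStats is an unfinished random-roll function that never runs.
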(event `self.ReceiveBeginPlay`
  (bind _returnvalue (`|GetDataTableRow` "/Game/Blueprints/Data/DataTable/EnemyDataTable.EnemyDataTable" "1000")
    (:`then`
      (bind (_name _initialvalue _basevital _basestr _basetgh _basedex) (break `/Game/Blueprints/Data/BP_EnemyDataTableType` _returnvalue))
      (bind _returnvalue_2 (`self.PointStats` (`|MakeArray` (`KismetMathLibrary.FTrunc` _basevital) (`KismetMathLibrary.FTrunc` _basestr) (`KismetMathLibrary.FTrunc` _basetgh) (`KismetMathLibrary.FTrunc` _basedex)))
        (:`True`
          (for _array_element _returnvalue_2
            (`KismetSystemLibrary.PrintString` (`KismetStringLibrary.Conv_IntToString` _array_element))))))))

(fn `UserConstructionScript`)