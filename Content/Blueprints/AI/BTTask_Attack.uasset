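; Behavior tree task that picks an attack target for an AI enemy, without dealing damage itself.
; On execute it flips a coin between the game mode's player and pet arrays, stores a random entry as TargetPawn and finishes successfully.
; The random index for players is bounded by PetMax and for pets by PlayerMax.
; An unconnected branch sketches lowest-HP targeting from HP bar values but never runs.
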(event `self.ReceiveExecuteAI`
  (params (OwnerController :type "AIController Object Reference") (ControlledPawn :type "Pawn Object Reference"))
  (bind _gamemode_ref (`self.Gamemode_Ref`))
  (set `self.Owner_Enemy` ControlledPawn)
  (bind _asbp_first_person_game_mode (cast `/Game/Blueprints/FirstPersonBP/BP_FirstPersonGameMode` (`GameplayStatics.GetGameMode`)))
  (set `self.Gamemode_Ref` _asbp_first_person_game_mode)
  (if (`KismetMathLibrary.RandomBool`)
    (set `self.Target_Pawn` (`|GetArrayItem` (`/Game/Blueprints/FirstPersonBP/BP_FirstPersonGameMode.PlayerS` _gamemode_ref) (`KismetMathLibrary.RandomInteger` (`/Game/Blueprints/FirstPersonBP/BP_FirstPersonGameMode.PetMax` _gamemode_ref))))
    (else
      (set `self.Target_Pawn` (`|GetArrayItem` (`/Game/Blueprints/FirstPersonBP/BP_FirstPersonGameMode.PetS` _gamemode_ref) (`KismetMathLibrary.RandomInteger` (`/Game/Blueprints/FirstPersonBP/BP_FirstPersonGameMode.PlayerMax` _gamemode_ref))))))
  (`self.FinishExecute` true))