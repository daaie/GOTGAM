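; AI controller for an enemy that hands its decisions to a behavior tree.
; On possess it applies the BTB_Enemy blackboard, runs BTT_Enemy, then calls InitEnemyState on the pawn if it is a TestAI_Enemy.
; An unconnected, never-executed block sketches turn-based action choice: a weighted roll writes either the attack key or both defence and run keys to the blackboard, then clears turn flags.
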(event `self.OnPossess`
  (params (PossessedPawn :type "Pawn Object Reference"))
  (`|ExecutionSequence`
    (:`then_0`
      (`self.UseBlackboard` "/Game/Blueprints/AI/BTB_Enemy.BTB_Enemy"))
    (:`then_1`
      (`self.RunBehaviorTree` "/Game/Blueprints/AI/BTT_Enemy.BTT_Enemy"))
    (:`then_2`
      (bind _astest_ai_enemy (cast `/Game/Blueprints/Battle/TestAI_Enemy` (`self.K2_GetPawn`)))
      (`/Game/Blueprints/Battle/TestAI_Enemy.InitEnemyState` _astest_ai_enemy))))

(fn `UserConstructionScript`)