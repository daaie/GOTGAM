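; Field zone that rolls for random enemy encounters while the player moves inside its box.
; Entering the box sets IsBattle and starts a looping one-second timer; leaving only clears the flag, without stopping the timer.
; Each tick, if the field character's IsMInDistance flag is set, it makes a weighted 25% roll and resets that flag.
; Success calls EnemyBattle, currently a debug-print placeholder for the battle system.
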(event `Enemy Battle`
  ;[1 1 1] 배틀 시작 이벤트입니다 여기다가 배틀 시스템 넣어주세요
  (`KismetSystemLibrary.PrintString` "Start")
  (set `self.IsBattle?` true)
  (`KismetSystemLibrary.Delay` 1.0))

(event `self.Box.OnComponentBeginOverlap`
  (params (OverlappedComponent :type "PrimitiveComponent Object Reference") (OtherActor :type "Actor Object Reference") (OtherComp :type "PrimitiveComponent Object Reference") (OtherBodyIndex :type Integer) (bFromSweep :type Boolean) (SweepResult :type "HitResult Structure (by ref)"))
  ;[1 1 1] 몬스터 출연지역에 들어가게 되면 작동합니다.
  (`KismetSystemLibrary.PrintString` "In")
  (set `self.IsBattle?` true)
  (set `self.PlayerRef` OtherActor)
  (`KismetSystemLibrary.K2_SetTimerDelegate` (delegate `Battle Probability`) 1.0 true))

(event `self.Box.OnComponentEndOverlap`
  (params (OverlappedComponent :type "PrimitiveComponent Object Reference") (OtherActor :type "Actor Object Reference") (OtherComp :type "PrimitiveComponent Object Reference") (OtherBodyIndex :type Integer))
  ;[1 1 1] 몬스터 출연지역에 들어가게 되면 작동합니다.
  (`KismetSystemLibrary.PrintString` "Out")
  (set `self.IsBattle?` false))

(event `Battle Probability`
  ;[1 1 1] 지역을 많이 이동할 수록 출연률이 올라갑니다.
  (if (`self.IsBattle?`)
    (bind _asbp_field_controller (cast `/Game/Blueprints/Field/BP_FieldController` (`GameplayStatics.GetPlayerController` 0)))
    (`/Engine/EditorBlueprintResources/StandardMacros.IsValid` _asbp_field_controller
      (:`Is Valid`
        (bind _asbp_field_character (cast `/Game/Blueprints/Field/BP_FieldCharacter` (`Controller.K2_GetPawn` _asbp_field_controller)))
        (`/Engine/EditorBlueprintResources/StandardMacros.IsValid` _asbp_field_character
          (:`Is Valid`
            (if (`/Game/Blueprints/Field/BP_FieldCharacter.IsMInDistance?` _asbp_field_character)
              (if (`KismetMathLibrary.RandomBoolWithWeight` 0.25)
                (`KismetSystemLibrary.PrintString` "Success")
                (`self.Enemy Battle`)
                (else
                  (`KismetSystemLibrary.PrintString` "fail")))
              (set `/Game/Blueprints/Field/BP_FieldCharacter.IsMInDistance?` false _asbp_field_character))))))))

(fn `UserConstructionScript`)