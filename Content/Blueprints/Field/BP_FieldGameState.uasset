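; Field game state that syncs the player's character and pet stats with a PHP web backend through HTTP POST requests keyed by UserID.
; On BeginPlay, only non-authority instances request both stat sets, using the GameInstance URL, and parse the JSON replies into Stat and the PetStat array.
; Update events post stats using field-name arrays.
; Character updates re-fetch afterward, while pet updates ignore the response.
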(event `self.ReceiveBeginPlay`
  (bind _asgame_instance (cast `/Game/Blueprints/AllLevels/GameInstance` (`GameplayStatics.GetGameInstance`)))
  (set `self.GameInstanceRef` _asgame_instance)
  (set `self.URL` (`/Game/Blueprints/AllLevels/GameInstance.URL` (`self.GameInstanceRef`)))
  (`/Engine/EditorBlueprintResources/ActorMacros.Switch Has Authority`
    (:`Remote`
      (`|ExecutionSequence`
        (:`then_0`
          (`self.SelectCharacterStatus`))
        (:`then_1`
          (`self.SelectPetStatus`))))))

(event `SelectCharacterStatus`
  ;[1 1 1] SelectCharacter
  (bind _output_get (set `self.Request` (`VaRestRequestJSON.ConstructRequestExt` "POST" "x_www_form_urlencoded_body")))
  (bind _returnvalue (`VaRestRequestJSON.GetRequestObject` _output_get))
  (set `self.RequestObject` _returnvalue)
  (`VaRestJsonObject.SetStringField` (`self.RequestObject`) "userid" (`/Game/Blueprints/AllLevels/GameInstance.UserID` (`self.GameInstanceRef`)))
  (`VaRestJsonObject.SetStringField` (`self.RequestObject`) "action" "character")
  (add `VaRestRequestJSON.OnRequestComplete` (`self.Request`) (delegate `SelectCharacterInfo`))
  (`VaRestRequestJSON.ProcessURL` (`self.Request`) (`KismetStringLibrary.Concat_StrStr` (`self.URL`) "/SelectStatus.php")))

(event `SelectCharacterInfo`
  (params (Request :type "VaRestRequestJSON Object Reference"))
  (bind _selectfieldname (`self.SelectFieldName`))
  ;[1 1 1] SelectCharacter
  (bind _returnvalue (`VaRestRequestJSON.GetResponseObject` Request))
  (set `self.Json` _returnvalue)
  (if (`VaRestJsonObject.GetBoolField` (`self.Json`) "Success")
    (while (< (`self.SelectIndex`) (`KismetArrayLibrary.Array_Length` _selectfieldname))
      (`KismetArrayLibrary.Array_Set` (`self.SelectFieldValue`) (`self.SelectIndex`) (`VaRestJsonObject.GetStringField` (`self.Json`) (`|GetArrayItem` _selectfieldname (`self.SelectIndex`))))
      (`/Engine/EditorBlueprintResources/StandardMacros.IncrementInt` (`self.SelectIndex`)))
    (set `self.Stat` (make `/Game/Blueprints/AllLevels/CharacterStat` (`self.NewMacro_0` 12) (`KismetStringLibrary.Conv_StringToInt` (`self.NewMacro_0` 0)) (`KismetStringLibrary.Conv_StringToDouble` (`self.NewMacro_0` 6)) (`KismetStringLibrary.Conv_StringToDouble` (`self.NewMacro_0` 11)) (`KismetStringLibrary.Conv_StringToDouble` (`self.NewMacro_0` 7)) (`KismetStringLibrary.Conv_StringToDouble` (`self.NewMacro_0` 8)) (`KismetStringLibrary.Conv_StringToDouble` (`self.NewMacro_0` 9)) (`KismetStringLibrary.Conv_StringToInt` (`self.NewMacro_0` 10)) (`KismetStringLibrary.Conv_StringToInt` (`self.NewMacro_0` 2)) (`KismetStringLibrary.Conv_StringToInt` (`self.NewMacro_0` 3)) (`KismetStringLibrary.Conv_StringToInt` (`self.NewMacro_0` 4)) (`KismetStringLibrary.Conv_StringToInt` (`self.NewMacro_0` 5)) (`self.NewMacro_0` 1) (`KismetStringLibrary.Conv_StringToInt` (`self.NewMacro_0` 13)) (`KismetStringLibrary.Conv_StringToInt` (`self.NewMacro_0` 14))))
    (set `self.SelectIndex` 0)
    (else
      (`KismetSystemLibrary.PrintString` "캐릭터 정보 로딩실패"))))

(event `SelectPetStatus`
  ;[1 1 1] SelectPet
  (bind _output_get (set `self.Request` (`VaRestRequestJSON.ConstructRequestExt` "POST" "x_www_form_urlencoded_body")))
  (bind _returnvalue (`VaRestRequestJSON.GetRequestObject` _output_get))
  (set `self.RequestObject` _returnvalue)
  (`VaRestJsonObject.SetStringField` (`self.RequestObject`) "userid" (`/Game/Blueprints/AllLevels/GameInstance.UserID` (`self.GameInstanceRef`)))
  (`VaRestJsonObject.SetStringField` (`self.RequestObject`) "action" "pet")
  (add `VaRestRequestJSON.OnRequestComplete` (`self.Request`) (delegate `SelectPet`))
  (`VaRestRequestJSON.ProcessURL` (`self.Request`) (`KismetStringLibrary.Concat_StrStr` (`self.URL`) "/SelectStatus.php")))

(event `SelectPet`
  (params (Request :type "VaRestRequestJSON Object Reference"))
  ;[1 1 1] SelectPet
  (bind _returnvalue (`VaRestRequestJSON.GetResponseObject` Request))
  (bind _output_get (set `self.JsonPet` _returnvalue))
  (bind _returnvalue_2 (`VaRestJsonObject.GetObjectArrayField` _output_get "PetResults"))
  (set `self.NumPet` (`KismetArrayLibrary.Array_Length` _returnvalue_2))
  (while (< (`self.PetIndex`) (`self.NumPet`))
    (bind _output (`|GetArrayItem` _returnvalue_2 (`self.PetIndex`)))
    (`KismetArrayLibrary.Array_Set` (`self.PetStat`) (`self.PetIndex`) (make `/Game/Blueprints/AllLevels/PetStat` (`KismetStringLibrary.Conv_StringToInt` (`VaRestJsonObject.GetStringField` _output "pet_id")) (`VaRestJsonObject.GetStringField` _output "pet_name") (`KismetStringLibrary.Conv_StringToInt` (`VaRestJsonObject.GetStringField` _output "level")) (`KismetStringLibrary.Conv_StringToDouble` (`VaRestJsonObject.GetStringField` _output "exp")) (`KismetStringLibrary.Conv_StringToDouble` (`VaRestJsonObject.GetStringField` _output "current_vital")) (`KismetStringLibrary.Conv_StringToDouble` (`VaRestJsonObject.GetStringField` _output "vital")) (`KismetStringLibrary.Conv_StringToDouble` (`VaRestJsonObject.GetStringField` _output "str")) (`KismetStringLibrary.Conv_StringToDouble` (`VaRestJsonObject.GetStringField` _output "tgh")) (`KismetStringLibrary.Conv_StringToDouble` (`VaRestJsonObject.GetStringField` _output "dex")) (`VaRestJsonObject.GetStringField` _output "status") (`VaRestJsonObject.GetStringField` _output "skill")))
    (`/Engine/EditorBlueprintResources/StandardMacros.IncrementInt` (`self.PetIndex`)))
  (set `self.PetIndex` 0))

(event `UpdateCharacterStat`
  (bind (_stat_name _stat_level _stat_vital _stat_exp _stat_str _stat_tgh _stat_dex _stat_attr _stat_stamina _stat_power _stat_health _stat_elabo _stat_gender _stat_currentvital _stat_statepoint) (break `/Game/Blueprints/AllLevels/CharacterStat` (`self.Stat`)))
  ;[1 1 1] UpdateCharacter
  (bind _output_get (set `self.Request` (`VaRestRequestJSON.ConstructRequestExt` "POST" "x_www_form_urlencoded_body")))
  (bind _returnvalue (`VaRestRequestJSON.GetRequestObject` _output_get))
  (set `self.RequestObject` _returnvalue)
  (`VaRestJsonObject.SetStringField` (`self.RequestObject`) "userid" (`/Game/Blueprints/AllLevels/GameInstance.UserID` (`self.GameInstanceRef`)))
  (for (_array_element _array_index) (`self.UpdateStat`)
    (`VaRestJsonObject.SetStringField` (`self.RequestObject`) _array_element (`KismetStringLibrary.Conv_IntToString` (`|GetArrayItem` (`|MakeArray` _stat_level _stat_attr _stat_stamina _stat_power _stat_health _stat_elabo _stat_currentvital _stat_statepoint) _array_index))))
  (add `VaRestRequestJSON.OnRequestComplete` (`self.Request`) (delegate `UpdateCharacter`))
  (`VaRestRequestJSON.ProcessURL` (`self.Request`) (`KismetStringLibrary.Concat_StrStr` (`self.URL`) "/UpdateCharacterStatus.php")))

(event `UpdateCharacter`
  (params (Request :type "VaRestRequestJSON Object Reference"))
  ;[1 1 1] UpdateCharacter
  (`self.SelectCharacterStatus`))

(event `UpdatePet`
  (params (PetIndex :type Integer))
  (bind _requestobject (`self.RequestObject`))
  (bind (_output_pet_id _output_name _output_level _output_exp _output_current_vital _output_vital _output_str _output_tgh _output_dex _output_status) (break `/Game/Blueprints/AllLevels/PetStat` (`|GetArrayItem` (`self.PetStat`) PetIndex)))
  ;[1 1 1] UpdatePet
  (bind _output_get (set `self.Request` (`VaRestRequestJSON.ConstructRequestExt` "POST" "x_www_form_urlencoded_body")))
  (bind _returnvalue (`VaRestRequestJSON.GetRequestObject` _output_get))
  (set `self.RequestObject` _returnvalue)
  (`VaRestJsonObject.SetStringField` _requestobject "userid" (`/Game/Blueprints/AllLevels/GameInstance.UserID` (`self.GameInstanceRef`)))
  (`VaRestJsonObject.SetStringField` _requestobject "name" _output_name)
  (`VaRestJsonObject.SetStringField` _requestobject "status" _output_status)
  (for (_array_element _array_index) (`self.UpdatePetStat`)
    (`VaRestJsonObject.SetStringField` (`self.RequestObject`) _array_element (`KismetStringLibrary.Conv_DoubleToString` (`|GetArrayItem` (`|MakeArray` (`KismetMathLibrary.Conv_IntToDouble` _output_level) _output_exp _output_current_vital _output_vital _output_str _output_tgh _output_dex) _array_index))))
  (add `VaRestRequestJSON.OnRequestComplete` (`self.Request`) (delegate `CustomEvent_1`))
  (`VaRestRequestJSON.ProcessURL` (`self.Request`) (`KismetStringLibrary.Concat_StrStr` (`self.URL`) "/UpdatePetStatus.php")))

(event `CustomEvent_1`
  (params (Request :type "VaRestRequestJSON Object Reference"))
  ;[1 1 1] UpdatePet
)

(fn `UserConstructionScript`)