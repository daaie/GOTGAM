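; Field game mode that handles player login, respawn and parties of up to four players.
; BeginPlay caches enemy spawn locations; PostLogin calls ClientLogin and sets the controller's UserID; respawn replaces the pawn at the world origin.
; Parties are structs of controllers in PartyPlayers, with the array index as party number and Party1 as owner.
; Create, add and leave events lead to PartyRefrash, which copies party data and owner pawn to members, while disband removes the entry.
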(event `self.ReceiveBeginPlay`
  ;[1 1 1] BeginPlay
  (`self.SpawnArea`))

(event `SpawnArea`
  ;[1 1 1] SpawnArea소환?!
  (bind _outactors (`GameplayStatics.GetAllActorsOfClass` "/Game/Blueprints/Field/BP_EnemySpawnLocation.BP_EnemySpawnLocation_C"))
  (set `self.EnemySpawnArea` _outactors))

(event `self.K2_PostLogin`
  (params (NewPlayer :type "PlayerController Object Reference"))
  (bind _userid (`self.UserID`))
  ;[1 1 1] OnPostLogin
  (bind _asbp_field_controller (cast `/Game/Blueprints/Field/BP_FieldController` NewPlayer))
  (`/Game/Blueprints/Field/BP_FieldController.ClientLogin` _asbp_field_controller _asbp_field_controller)
  (`KismetSystemLibrary.PrintString` _userid)
  (set `/Game/Blueprints/Field/BP_FieldController.UserID` _userid _asbp_field_controller))

(event `RespawnPlayer`
  (params (PlayerController :type "PlayerController Object Reference"))
  (bind _returnvalue (`Controller.K2_GetPawn` PlayerController))
  ;[1 1 1] 캐릭터Respawn
  (`/Engine/EditorBlueprintResources/StandardMacros.IsValid` _returnvalue
    (:`Is Valid`
      (`self.K2_DestroyActor` _returnvalue)
      (bind _returnvalue_2 (`|SpawnActorFromClass` "/Game/Blueprints/Field/BP_FieldCharacter.BP_FieldCharacter_C" (`KismetMathLibrary.MakeTransform` (0.0 0.0 0.0)) "AdjustIfPossibleButAlwaysSpawn" "OverrideRootScale" null null))
      (`Controller.Possess` PlayerController _returnvalue_2)
      (`KismetSystemLibrary.PrintString` "Hello"))))

(event `CreatePartyGM`
  (params (PC_HostPlayer :type "/Game/Blueprints/Field/BP_FieldController Object Reference") (PC_OtherPlayer :type "/Game/Blueprints/Field/BP_FieldController Object Reference"))
  ;[1 1 1] 파티생성
  (`/Engine/EditorBlueprintResources/StandardMacros.IsValid` PC_HostPlayer
    (:`Is Valid`
      (bind _returnvalue (`KismetArrayLibrary.Array_Add` (`self.PartyPlayers`) (make `/Game/Blueprints/Field/Party` PC_HostPlayer)))
      (`self.party add playerGM` _returnvalue PC_OtherPlayer)
      (set `/Game/Blueprints/Field/BP_FieldController.PartyNumber` _returnvalue PC_HostPlayer)
      (set `/Game/Blueprints/Field/BP_FieldController.IsPartyInvate?` true PC_HostPlayer)
      (set `/Game/Blueprints/Field/BP_FieldController.IsPartyOwner?` true PC_HostPlayer))
    (:`Is Not Valid`
      (`KismetSystemLibrary.PrintString` "Error: Host Player Null"))))

(event `Party add playerGM`
  (params (PartyNumber :type Integer) (PC_OtherPlayer :type "/Game/Blueprints/Field/BP_FieldController Object Reference"))
  (bind _partyplayers (`self.PartyPlayers`))
  (bind (_output_party1 _output_party2 _output_party3 _output_party4) (break `/Game/Blueprints/Field/Party` (`|GetArrayItem` (`self.PartyPlayers`) PartyNumber)))
  ;[1 1 1] 파티원 추가
  (`/Engine/EditorBlueprintResources/StandardMacros.IsValid` PC_OtherPlayer
    (:`Is Valid`
      (`/Engine/EditorBlueprintResources/StandardMacros.IsValid` _output_party2
        (:`Is Valid`
          (`/Engine/EditorBlueprintResources/StandardMacros.IsValid` _output_party3
            (:`Is Valid`
              (`/Engine/EditorBlueprintResources/StandardMacros.IsValid` _output_party4
                (:`Is Not Valid`
                  (`KismetArrayLibrary.Array_Set` _partyplayers PartyNumber (make `/Game/Blueprints/Field/Party` _output_party1 _output_party2 _output_party3 PC_OtherPlayer)))))
            (:`Is Not Valid`
              (`KismetArrayLibrary.Array_Set` _partyplayers PartyNumber (make `/Game/Blueprints/Field/Party` _output_party1 _output_party2 PC_OtherPlayer)))))
        (:`Is Not Valid`
          (`KismetArrayLibrary.Array_Set` _partyplayers PartyNumber (make `/Game/Blueprints/Field/Party` _output_party1 PC_OtherPlayer))))
      (set `/Game/Blueprints/Field/BP_FieldController.PartyNumber` PartyNumber PC_OtherPlayer)
      (set `/Game/Blueprints/Field/BP_FieldController.IsPartyInvate?` true PC_OtherPlayer)
      (`self.PartyRefrash` PartyNumber))
    (:`Is Not Valid`
      (`KismetSystemLibrary.PrintString` "Error: Other Player Null"))))

(event `DestroyPartyGM`
  (params (PC_HostPlayer :type "/Game/Blueprints/Field/BP_FieldController Object Reference") (PartyNumber :type Integer))
  (bind (_output_party1 _output_party2 _output_party3 _output_party4) (break `/Game/Blueprints/Field/Party` (`|GetArrayItem` (`self.PartyPlayers`) PartyNumber)))
  ;[1 1 1] 파티장이 파티를 해제
  (`/Engine/EditorBlueprintResources/StandardMacros.IsValid` PC_HostPlayer
    (:`Is Valid`
      (`/Engine/EditorBlueprintResources/StandardMacros.IsValid` _output_party2
        (:`Is Valid`
          (set `/Game/Blueprints/Field/BP_FieldController.PartyArray` (struct) _output_party2)
          (set `/Game/Blueprints/Field/BP_FieldController.IsPartyInvate?` false _output_party2)
          (`/Game/Blueprints/Field/BP_FieldController.RemovePartyWidget` _output_party2))
        (:`Is Not Valid`
          _))
      (`/Engine/EditorBlueprintResources/StandardMacros.IsValid` _output_party3
        (:`Is Valid`
          (set `/Game/Blueprints/Field/BP_FieldController.PartyArray` (struct) _output_party3)
          (set `/Game/Blueprints/Field/BP_FieldController.IsPartyInvate?` false _output_party3)
          (`/Game/Blueprints/Field/BP_FieldController.RemovePartyWidget` _output_party3))
        (:`Is Not Valid`
          _))
      (`/Engine/EditorBlueprintResources/StandardMacros.IsValid` _output_party4
        (:`Is Valid`
          (set `/Game/Blueprints/Field/BP_FieldController.PartyArray` (struct) _output_party4)
          (set `/Game/Blueprints/Field/BP_FieldController.IsPartyInvate?` false _output_party4)
          (`/Game/Blueprints/Field/BP_FieldController.RemovePartyWidget` _output_party4))
        (:`Is Not Valid`
          _))
      (`KismetArrayLibrary.Array_Remove` (`self.PartyPlayers`) PartyNumber)
      (set `/Game/Blueprints/Field/BP_FieldController.IsPartyInvate?` false PC_HostPlayer)
      (set `/Game/Blueprints/Field/BP_FieldController.IsPartyOwner?` false PC_HostPlayer))
    (:`Is Not Valid`
      (`KismetSystemLibrary.PrintString` "Error: Host Player Null"))))

(event `PartyEscapeGM`
  (params (PC_HostPlayer :type "/Game/Blueprints/Field/BP_FieldController Object Reference") (PartyNumber :type Integer))
  (bind _partyplayers (`self.PartyPlayers`))
  (bind (_output_party1 _output_party2 _output_party3 _output_party4) (break `/Game/Blueprints/Field/Party` (`|GetArrayItem` _partyplayers PartyNumber)))
  ;[1 1 1] 파티 탈퇴
  (`/Engine/EditorBlueprintResources/StandardMacros.IsValid` PC_HostPlayer
    (:`Is Valid`
      (if (== PC_HostPlayer _output_party2)
        (`KismetArrayLibrary.Array_Set` _partyplayers PartyNumber (make `/Game/Blueprints/Field/Party` _output_party1 null _output_party3 _output_party4))
        (set `/Game/Blueprints/Field/BP_FieldController.IsPartyInvate?` false PC_HostPlayer :!label _label)
        (`self.PartyRefrash` PartyNumber)
        (elif (== PC_HostPlayer _output_party3)
          (`KismetArrayLibrary.Array_Set` _partyplayers PartyNumber (make `/Game/Blueprints/Field/Party` _output_party1 _output_party2 null _output_party4))
          (goto _label)
          (elif (== PC_HostPlayer _output_party4)
            (`KismetArrayLibrary.Array_Set` _partyplayers PartyNumber (make `/Game/Blueprints/Field/Party` _output_party1 _output_party2 _output_party3))
            (goto _label)))))
    (:`Is Not Valid`
      (`KismetSystemLibrary.PrintString` "Error: Host Player Null"))))

(event `PartyRefrash`
  (params (PartyNumber :type Integer))
  (bind _partyplayers (`self.PartyPlayers`))
  (bind (_output_party1 _output_party2 _output_party3 _output_party4) (break `/Game/Blueprints/Field/Party` (`|GetArrayItem` _partyplayers PartyNumber)))
  (bind _output (`|GetArrayItem` _partyplayers PartyNumber))
  ;[1 1 1] 파티 정보값 새로 고침
  (bind _output_get (set `/Game/Blueprints/Field/BP_FieldController.PartyArray` _output _output_party1))
  (`self.PartyRefreshPawn` _output_get _output_party1)
  (`/Engine/EditorBlueprintResources/StandardMacros.IsValid` _output_party2
    (:`Is Valid`
      (bind _output_get_2 (set `/Game/Blueprints/Field/BP_FieldController.PartyArray` _output _output_party2))
      (`self.PartyRefreshPawn` _output_get_2 _output_party2))
    (:`Is Not Valid`
      _))
  (`/Engine/EditorBlueprintResources/StandardMacros.IsValid` _output_party3
    (:`Is Valid`
      (bind _output_get_3 (set `/Game/Blueprints/Field/BP_FieldController.PartyArray` _output _output_party3))
      (`self.PartyRefreshPawn` _output_get_3 _output_party3))
    (:`Is Not Valid`
      _))
  (`/Engine/EditorBlueprintResources/StandardMacros.IsValid` _output_party4
    (:`Is Valid`
      (bind _output_get_4 (set `/Game/Blueprints/Field/BP_FieldController.PartyArray` _output _output_party4))
      (`self.PartyRefreshPawn` _output_get_4 _output_party4))))

(event `PartyRefreshPawn`
  (params (Party :type "/Game/Blueprints/Field/Party Structure") (PlayerController :type "/Game/Blueprints/Field/BP_FieldController Object Reference"))
  (bind _asbp_field_character (cast `/Game/Blueprints/Field/BP_FieldCharacter` (`Controller.K2_GetPawn` (`.Party1_14_A25AD661429ADA62638E61A3E6DB14B7` (break `/Game/Blueprints/Field/Party` Party)))))
  (`/Engine/EditorBlueprintResources/StandardMacros.IsValid` _asbp_field_character
    (:`Is Valid`
      (set `/Game/Blueprints/Field/BP_FieldController.PartyOwnerPawn` _asbp_field_character PlayerController))))

(fn `UserConstructionScript`)