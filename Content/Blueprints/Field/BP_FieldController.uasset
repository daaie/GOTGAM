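; Player controller for the multiplayer field map, handling login placement, chat, overhead names, click-to-move and parties of up to four.
; Stat saves and loads go through the field GameState; party stats come from an HTTP request.
; Clicking another character briefly highlights it and pairs both controllers for invites, which the GameMode manages.
; Party leaders pull members along when moving and open a battle session that members join by the leader's ID.
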(event `C2S_LoginLocation`
  ;[1 1 1] 시작위치
  (bind _asbp_field_game_state (cast `/Game/Blueprints/Field/BP_FieldGameState` (`GameplayStatics.GetGameState`)))
  (`self.S2C_LoginLocation` self (`/Game/Blueprints/Field/BP_FieldGameState.Location` _asbp_field_game_state)))

(event `S2C_LoginLocation`
  (params (FieldPC :type "/Game/Blueprints/Field/BP_FieldController Object Reference") (Location :type "Vector Structure"))
  ;[1 1 1] 시작위치
  (`self.K2_SetActorLocation` (`self.K2_GetPawn` FieldPC) Location false false))

(event `GetPartyStat`
  (params (Name :type String))
  ;[1 1 1] Replicated stat 요청
  (bind _output_get (set `self.Request` (`VaRestRequestJSON.ConstructRequestExt` "POST" "x_www_form_urlencoded_body")))
  (bind _returnvalue (`VaRestRequestJSON.GetRequestObject` _output_get))
  (set `self.RequestObject` _returnvalue)
  (`VaRestJsonObject.SetStringField` (`self.RequestObject`) "userid" Name)
  (add `VaRestRequestJSON.OnRequestComplete` (`self.Request`) (delegate `Custom Event_0`))
  (bind _asgame_instance (cast `/Game/Blueprints/AllLevels/GameInstance` (`GameplayStatics.GetGameInstance`)))
  (`VaRestRequestJSON.ProcessURL` (`self.Request`) (`KismetStringLibrary.Concat_StrStr` (`/Game/Blueprints/AllLevels/GameInstance.URL` _asgame_instance) "/SelectPartyStat")))

(event `Custom Event_0`
  (params (Request :type "VaRestRequestJSON Object Reference"))
  (bind _json (`self.Json`))
  ;[1 1 1] Replicated stat 요청
  (bind _returnvalue (`VaRestRequestJSON.GetResponseObject` Request))
  (set `self.Json` _returnvalue)
  (if (`VaRestJsonObject.GetBoolField` (`self.Json`) "Success")
    (set `self.PartyStat` (make `/Game/Blueprints/Field/PartyStat` (`VaRestJsonObject.GetStringField` _json "NickName") (`KismetStringLibrary.Conv_StringToInt` (`VaRestJsonObject.GetStringField` _json "Level"))))))

(event `self.ReceiveBeginPlay`
  ;[1 1 1] 위젯 설정
  (`self.S2C_SetupWidget`)
  (`self.S2A_PlayerControllerUserName`)
  (`/Engine/EditorBlueprintResources/ActorMacros.Switch Has Authority`
    (:`Remote`
      (`self.C2S_LoginLocation`))))

(event `LogOut`
  (params (FieldPC :type "/Game/Blueprints/Field/BP_FieldController Object Reference"))
  ;[1 1 1] OnLogon/Logout
  (bind _asbp_field_game_state (cast `/Game/Blueprints/Field/BP_FieldGameState` (`GameplayStatics.GetGameState`)))
  (`/Game/Blueprints/Field/BP_FieldGameState.UpdateCharacterStat` _asbp_field_game_state FieldPC))

(event `SelectCharacterStat`
  (params (FieldPC :type "/Game/Blueprints/Field/BP_FieldController Object Reference"))
  ;[1 1 1] OnLogon/Logout
  (bind _asbp_field_game_state (cast `/Game/Blueprints/Field/BP_FieldGameState` (`GameplayStatics.GetGameState`)))
  (`/Game/Blueprints/Field/BP_FieldGameState.SelectCharacterStatus` _asbp_field_game_state FieldPC))

(event `S2C_SetupWidget`
  ;[1 1 1] 리플리케이트 웨젯 설정 클라이언트에서 실행
  (bind _returnvalue (`|CreateWidget` "/Game/UMG/Field/Server/UMG_ChatWidget.UMG_ChatWidget_C" self))
  (bind _output_get (set `self.ChatWidget` _returnvalue))
  (`UserWidget.AddToViewport` _output_get 0)
  (`Widget.SetUserFocus` _output_get self))

(event `SetCharacterStatus`
  (params (Stat :type "/Game/Blueprints/AllLevels/CharacterStat Structure") (Stone :type Integer) (location :type "Vector Structure"))
  ;[1 1 1] OnLogon/Logout
  (bind _asbp_field_game_state (cast `/Game/Blueprints/Field/BP_FieldGameState` (`GameplayStatics.GetGameState`)))
  (`/Game/Blueprints/Field/BP_FieldGameState.SetCharacterStatus` _asbp_field_game_state Stat Stone location))

(event `ServerPawn`
  (bind (_partyarray_party1 _partyarray_party2 _partyarray_party3 _partyarray_party4) (break `/Game/Blueprints/Field/Party` (`self.PartyArray`)))
  ;[1 1 1] 파티 기차놀이
  (if (== self _partyarray_party1)
    (bind _asbp_field_character (cast `/Game/Blueprints/Field/BP_FieldCharacter` (`self.K2_GetPawn` self)))
    (`/Game/Blueprints/Field/BP_FieldCharacter.MouseCursorPoint` _asbp_field_character)
    (`/Engine/EditorBlueprintResources/StandardMacros.IsValid` _partyarray_party2
      (:`Is Valid`
        (`self.PawnTrain` _partyarray_party2))
      (:`Is Not Valid`
        _))
    (`/Engine/EditorBlueprintResources/StandardMacros.IsValid` _partyarray_party3
      (:`Is Valid`
        (`self.PawnTrain` _partyarray_party3))
      (:`Is Not Valid`
        _))
    (`/Engine/EditorBlueprintResources/StandardMacros.IsValid` _partyarray_party4
      (:`Is Valid`
        (`self.PawnTrain` _partyarray_party4)))))

(event `S2A_PlayerControllerUserName`
  ;[1 1 1] 유저 이름 show
  ;;[1 1 1] 모든 유저를 찾은후 이름 함수 실행
  (bind _outactors (`GameplayStatics.GetAllActorsOfClass` "/Script/Engine.PlayerController"))
  (for _index (range (+ (`KismetArrayLibrary.Array_Length` _outactors) 1))
    (bind _asbp_field_controller (cast `/Game/Blueprints/Field/BP_FieldController` (`|GetArrayItem` _outactors _index)))
    (`/Engine/EditorBlueprintResources/StandardMacros.IsValid` _asbp_field_controller
      (:`Is Valid`
        (`self.S2A_UserName` _asbp_field_controller)))))

(event `C2S_SendChatMessage`
  (params (Message :type Text))
  ;[1 1 1] 채팅 값을 Controller를 이용하여 서버로 전송
  (bind _outactors (`GameplayStatics.GetAllActorsOfClass` "/Script/Engine.PlayerController"))
  (for _index (range (+ (`KismetArrayLibrary.Array_Length` _outactors) 1))
    (bind _asbp_field_controller (cast `/Game/Blueprints/Field/BP_FieldController` (`|GetArrayItem` _outactors _index)))
    (`/Engine/EditorBlueprintResources/StandardMacros.IsValid` _asbp_field_controller
      (:`Is Valid`
        (`self.S2A_AddChatMessage` _asbp_field_controller Message)))))

(event `UpdateCharacterInfo`
  (params (FieldPC :type "/Game/Blueprints/Field/BP_FieldController Object Reference"))
  ;[1 1 1] OnLogon/Logout
  (bind _asbp_field_game_state (cast `/Game/Blueprints/Field/BP_FieldGameState` (`GameplayStatics.GetGameState`)))
  (`/Game/Blueprints/Field/BP_FieldGameState.SelectCharacterStatus` _asbp_field_game_state FieldPC))

(event `S2A_UserName`
  ;[1 1 1] 유저 이름 show
  (bind _outactors (`GameplayStatics.GetAllActorsOfClass` "/Game/Blueprints/Field/BP_FieldCharacter.BP_FieldCharacter_C"))
  (for _index (range (+ (`KismetArrayLibrary.Array_Length` _outactors) 1))
    (bind _output (`|GetArrayItem` _outactors _index))
    (`/Engine/EditorBlueprintResources/StandardMacros.IsValid` _output
      (:`Is Valid`
        (`self.C2S_SearchName` _output)))))

(event `CreateBattleMap`
  (params (FieldPC :type "/Game/Blueprints/Field/BP_FieldController Object Reference"))
  ;[1 1 1] ServerTravelTest
  (`/Engine/EditorBlueprintResources/StandardMacros.IsValid` FieldPC
    (:`Is Valid`
      (bind _asgame_instance (cast `/Game/Blueprints/AllLevels/GameInstance` (`GameplayStatics.GetGameInstance`)))
      (set `GameInstanceBase.SessionName` (`KismetStringLibrary.Conv_StringToName` (`/Game/Blueprints/AllLevels/GameInstance.UserID` _asgame_instance)) _asgame_instance)
      (if (`/Game/Blueprints/Field/BP_FieldController.IsPartyInvate?` FieldPC)
        (if (`/Game/Blueprints/Field/BP_FieldController.IsPartyOwner?` FieldPC)
          (`GameInstanceBase.OpenBattleMap` _asgame_instance)
          (`self.SelectParty` FieldPC))))))

(event `PawnTrain`
  ;[1 1 1] 파티 기차놀이
  (bind _asbp_field_character (cast `/Game/Blueprints/Field/BP_FieldCharacter` (`self.K2_GetPawn`)))
  (`/Game/Blueprints/Field/BP_FieldCharacter.PartyTrain` _asbp_field_character))

(event `S2A_AddChatMessage`
  (params (Message :type Text))
  (bind _chatwidget (`self.ChatWidget`))
  ;[1 1 1] 클라이언트에서 채팅메시지 추가
  (`/Engine/EditorBlueprintResources/StandardMacros.IsValid` _chatwidget
    (:`Is Valid`
      (`/Game/UMG/Field/Server/UMG_ChatWidget.AddChatMessage` _chatwidget Message))))

(event `SelectParty`
  (params (FieldPC_PartyOwner :type "/Game/Blueprints/Field/BP_FieldController Object Reference"))
  (bind (_partyarray_party1 _partyarray_party2 _partyarray_party3 _partyarray_party4) (break `/Game/Blueprints/Field/Party` (`/Game/Blueprints/Field/BP_FieldController.PartyArray` FieldPC_PartyOwner)))
  (bind _userid (`/Game/Blueprints/Field/BP_FieldController.UserID` _partyarray_party1))
  ;[1 1 1] ServerTravelTest
  (`/Engine/EditorBlueprintResources/StandardMacros.IsValid` _partyarray_party2
    (:`Is Valid`
      (`self.JoinBattleMap` _partyarray_party2 _userid)
      (`/Engine/EditorBlueprintResources/StandardMacros.IsValid` _partyarray_party3
        (:`Is Valid`
          (`self.JoinBattleMap` _partyarray_party3 _userid)
          (`/Engine/EditorBlueprintResources/StandardMacros.IsValid` _partyarray_party4
            (:`Is Valid`
              (`self.JoinBattleMap` _partyarray_party4 _userid))))))))

(event `C2S_SearchName`
  (params (Character :type "/Game/Blueprints/Field/BP_FieldCharacter Object Reference"))
  ;[1 1 1] 유저 이름 show
  (bind _asbp_field_controller (cast `/Game/Blueprints/Field/BP_FieldController` (`Pawn.GetController` Character)))
  (bind _partystat_name (break `/Game/Blueprints/Field/PartyStat` (`/Game/Blueprints/Field/BP_FieldController.PartyStat` _asbp_field_controller)))
  (`self.S2A_UserNameWidgetshow` (`KismetTextLibrary.Conv_StringToText` _partystat_name) Character))

(event `Key|LeftMouseButton`
  (params (Key :type "Key Structure"))
  (:`Pressed`
    (`self.GetParticipantUnderCursor`)))

(event `S2A_UserNameWidgetshow`
  (params (Username :type Text) (Character :type "/Game/Blueprints/Field/BP_FieldCharacter Object Reference"))
  ;[1 1 1] 유저 이름 show
  (bind _asumg_user_name (cast `/Game/UMG/Field/UMG_UserName` (`WidgetComponent.GetUserWidgetObject` (`/Game/Blueprints/Field/BP_FieldCharacter.Widget` Character))))
  (`/Engine/EditorBlueprintResources/StandardMacros.IsValid` _asumg_user_name
    (:`Is Valid`
      (set `/Game/UMG/Field/UMG_UserName.UserNameWidget` Username _asumg_user_name))))

(event `JoinBattleMap`
  (params (Name :type String))
  ;[1 1 1] ServerTravelTest
  (bind _asgame_instance (cast `/Game/Blueprints/AllLevels/GameInstance` (`GameplayStatics.GetGameInstance`)))
  (set `GameInstanceBase.SessionName` (`KismetStringLibrary.Conv_StringToName` Name) _asgame_instance)
  (`GameInstanceBase.FindOnlineGames` _asgame_instance))

(event `GetParticipantUnderCursor`
  (bind (_hitresult _returnvalue) (`self.GetHitResultUnderCursorByChannel` "TraceTypeQuery3"))
  ;[1 1 1] 마우스 커서 위치 추적
  (set `self.TraceHitResult` _hitresult)
  (if _returnvalue
    ;[1 1 1] 케릭터 선택 결과 반환
    (bind _asbp_field_character (cast `/Game/Blueprints/Field/BP_FieldCharacter` (`.HitActor` (`GameplayStatics.BreakHitResult` (`self.TraceHitResult`))))
      (:`then`
        ;;[1 1 1] 현재 폰과 선택한 폰이 같을 경우 실행 X
        ;;;[1 1 1] result
        (bind _output_get (set `self.PlayerPawn` _asbp_field_character))
        (if (not (== _output_get (`self.K2_GetPawn` self)))
          (`self.GetsPlayerController` (`self.PlayerPawn`) self)
          (bind _mesh (`Character.Mesh` _output_get))
          ;;[1 1 1] 표면에 하이라이트 주는 부분(이쁘게 수정좀 ㅠㅠ;;)
          (`PrimitiveComponent.SetRenderCustomDepth` _mesh true)
          (`KismetSystemLibrary.Delay` 3.0)
          (`PrimitiveComponent.SetRenderCustomDepth` _mesh false)
          (`self.UnGetsPlayerController`)))
      (:`CastFailed`
        (bind _asbp_field_character_2 (cast `/Game/Blueprints/Field/BP_FieldCharacter` (`GameplayStatics.GetPlayerPawn` 0)))
        (if (`self.IsPartyInvate?`)
          (if (`self.IsPartyOwner?`)
            (`self.ServerPawn`))
          (else
            (`/Game/Blueprints/Field/BP_FieldCharacter.MouseCursorPoint` _asbp_field_character_2)))))
    (else
      (set `self.PlayerPawn` null))))

(event `GetsPlayerController`
  (params (PlayerPawn :type "/Game/Blueprints/Field/BP_FieldCharacter Object Reference") (HostController :type "/Game/Blueprints/Field/BP_FieldController Object Reference"))
  ;[1 1 1] 서버에서 플레이어 컨트롤러 찾기
  (bind _outactors (`GameplayStatics.GetAllActorsOfClass` "/Script/Engine.PlayerController"))
  (for _index (range (+ (`KismetArrayLibrary.Array_Length` _outactors) 1))
    (bind _output (`|GetArrayItem` _outactors _index))
    (`/Engine/EditorBlueprintResources/StandardMacros.IsValid` _output
      (:`Is Valid`
        (if (== (`self.K2_GetPawn` _output) PlayerPawn)
          (bind _asbp_field_controller (cast `/Game/Blueprints/Field/BP_FieldController` _output))
          (`/Engine/EditorBlueprintResources/StandardMacros.IsValid` _asbp_field_controller
            (:`Is Valid`
              (bind _output_get (set `self.HostPlayer` HostController))
              (bind _output_get_2 (set `self.OtherPlayer` _asbp_field_controller))
              (`self.GetReplicatedController` _output_get _output_get_2)
              (`self.GetReplicatedController` _output_get_2 _output_get _output_get_2))))))))

(event `UnGetsPlayerController`
  ;[1 1 1] 플레이어 컨트롤러 해제
  (set `self.HostPlayer` null)
  (set `self.OtherPlayer` null))

(event `GetReplicatedController`
  (params (Host :type "/Game/Blueprints/Field/BP_FieldController Object Reference") (Other :type "/Game/Blueprints/Field/BP_FieldController Object Reference"))
  ;[1 1 1] 코멘트
  (set `self.HostPlayer` Host)
  (set `self.OtherPlayer` Other))

(event `SetPartyArray`
  (params (NewParam :type "/Game/Blueprints/Field/Party Structure"))
  (bind _partystats (`self.PartyStats`))
  (bind _partystats_2 (`self.PartyStats`))
  ;[1 1 1] SetPartyArray
  (`KismetArrayLibrary.Array_Clear` (`self.PartyStats`))
  (`/Engine/EditorBlueprintResources/StandardMacros.IsValid` NewParam_Party1_14_A25AD661429ADA62638E61A3E6DB14B7
    (:`Is Valid`
      (`KismetArrayLibrary.Array_Add` _partystats (`/Game/Blueprints/Field/BP_FieldController.PartyStat` NewParam_Party1_14_A25AD661429ADA62638E61A3E6DB14B7))
      (`/Engine/EditorBlueprintResources/StandardMacros.IsValid` NewParam_Party2_16_268D2DB64DCE01DBAD49E685AA4ECC81
        (:`Is Valid`
          (`KismetArrayLibrary.Array_Add` _partystats (`/Game/Blueprints/Field/BP_FieldController.PartyStat` NewParam_Party2_16_268D2DB64DCE01DBAD49E685AA4ECC81))
          (`/Engine/EditorBlueprintResources/StandardMacros.IsValid` NewParam_Party3_17_2B91FF2F4BC28704BBFF11B9DD0DE643
            (:`Is Valid`
              (`KismetArrayLibrary.Array_Add` _partystats (`/Game/Blueprints/Field/BP_FieldController.PartyStat` NewParam_Party3_17_2B91FF2F4BC28704BBFF11B9DD0DE643))
              (`/Engine/EditorBlueprintResources/StandardMacros.IsValid` NewParam_Party4_18_D9E5280846DA5200FC34ABAB712345AA
                (:`Is Valid`
                  (`KismetArrayLibrary.Array_Add` _partystats (`/Game/Blueprints/Field/BP_FieldController.PartyStat` NewParam_Party4_18_D9E5280846DA5200FC34ABAB712345AA))
                  (`self.GetPartyArray` NewParam_Party1_14_A25AD661429ADA62638E61A3E6DB14B7 _partystats_2)
                  (`self.GetPartyArray` NewParam_Party2_16_268D2DB64DCE01DBAD49E685AA4ECC81 _partystats_2)
                  (`self.GetPartyArray` NewParam_Party3_17_2B91FF2F4BC28704BBFF11B9DD0DE643 _partystats_2)
                  (`self.GetPartyArray` NewParam_Party4_18_D9E5280846DA5200FC34ABAB712345AA _partystats_2))
                (:`Is Not Valid`
                  (`self.GetPartyArray` NewParam_Party1_14_A25AD661429ADA62638E61A3E6DB14B7 _partystats_2)
                  (`self.GetPartyArray` NewParam_Party2_16_268D2DB64DCE01DBAD49E685AA4ECC81 _partystats_2)
                  (`self.GetPartyArray` NewParam_Party3_17_2B91FF2F4BC28704BBFF11B9DD0DE643 _partystats_2))))
            (:`Is Not Valid`
              (`self.GetPartyArray` NewParam_Party2_16_268D2DB64DCE01DBAD49E685AA4ECC81 _partystats_2)
              (`self.GetPartyArray` NewParam_Party1_14_A25AD661429ADA62638E61A3E6DB14B7 _partystats_2))))
        (:`Is Not Valid`
          (`self.GetPartyArray` NewParam_Party1_14_A25AD661429ADA62638E61A3E6DB14B7 _partystats_2))))))

(event `Party_Fuction`
  (bind _hostplayer (`self.HostPlayer`))
  (bind _otherplayer (`self.OtherPlayer`))
  (bind _otherplayer_2 (`self.OtherPlayer`))
  ;[1 1 1] 파티 추가 기능
  (if (`self.IsPartyInvate?`)
    (`KismetSystemLibrary.PrintString` "이미 파티 입니다.")
    (else
      (bind _asbp_field_game_mode (cast `/Game/Blueprints/Field/BP_FieldGameMode` (`GameplayStatics.GetGameMode`)))
      (for (_array_element _array_index) (`/Game/Blueprints/Field/BP_FieldGameMode.PartyPlayers` _asbp_field_game_mode)
        (bind _returnvalue (== (`self.HostPlayer`) (`.Party1_14_A25AD661429ADA62638E61A3E6DB14B7` (break `/Game/Blueprints/Field/Party` _array_element))))
        (if _returnvalue
          (break)))
      (if _returnvalue
        (`/Game/Blueprints/Field/BP_FieldGameMode.Party add playerGM` _asbp_field_game_mode _array_index _otherplayer)
        (`self.PartyListWidget` _otherplayer)
        (else
          (`/Game/Blueprints/Field/BP_FieldGameMode.CreatePartyGM` _asbp_field_game_mode _hostplayer _otherplayer_2)
          (`self.PartyListWidget` _hostplayer)
          (`self.PartyListWidget` _otherplayer_2)))
      ;;[0 0 0] 변수 초기화
      (set `self.HostPlayer` null)
      (set `self.OtherPlayer` null)
      (bind _output_get (set `self.PartyArray` (`|GetArrayItem` (`/Game/Blueprints/Field/BP_FieldGameMode.PartyPlayers` _asbp_field_game_mode) (`self.PartyNumber`))))
      (`self.SetPartyArray` _output_get))))

(event `GetPartyArray`
  (params (NewParam :type "Array of /Game/Blueprints/Field/PartyStat Structure"))
  (bind _partywidget (`self.PartyWidget`))
  ;[1 1 1] 파티원 표시
  (`/Engine/EditorBlueprintResources/StandardMacros.IsValid` _partywidget
    (:`Is Valid`
      (`/Game/UMG/Field/UMG_Party.GetPartyArray` _partywidget NewParam))))

(event `UnParty_Function`
  (bind _partynumber (`self.PartyNumber`))
  ;[1 1 1] 파티 탈퇴
  (bind _asbp_field_game_mode (cast `/Game/Blueprints/Field/BP_FieldGameMode` (`GameplayStatics.GetGameMode`)))
  (if (== (`.Party1_14_A25AD661429ADA62638E61A3E6DB14B7` (break `/Game/Blueprints/Field/Party` (`|GetArrayItem` (`/Game/Blueprints/Field/BP_FieldGameMode.PartyPlayers` _asbp_field_game_mode) _partynumber))) self)
    (`/Game/Blueprints/Field/BP_FieldGameMode.DestroyPartyGM` _asbp_field_game_mode self _partynumber)
    (else
      (`/Game/Blueprints/Field/BP_FieldGameMode.PartyEscapeGM` _asbp_field_game_mode self _partynumber)))
  (set `self.PartyArray` (struct))
  (`self.RemovePartyWidget`))

(event `PartyInvateWidget`
  ;[1 1 1] 파티 초대 위젯 생성
  (bind _returnvalue (`|CreateWidget` "/Game/UMG/Field/Server/UMG_invateParty.UMG_invateParty_C" self))
  (`UserWidget.AddToViewport` _returnvalue 0))

(event `PartyEscapeWidget`
  (params (Text :type Text))
  ;[1 1 1] 파티 탈퇴 위젯 생성
  (bind _returnvalue (`|CreateWidget` "/Game/UMG/Field/Server/UMG_EscapeParty.UMG_EscapeParty_C" self))
  (set `/Game/UMG/Field/Server/UMG_EscapeParty.Text` Text _returnvalue)
  (`UserWidget.AddToViewport` _returnvalue 0))

(event `PartyListWidget`
  ;[1 1 1] 파티 리스트 위젯 생성 및 제거
  (bind _returnvalue (`|CreateWidget` "/Game/UMG/Field/UMG_Party.UMG_Party_C" self))
  (set `self.PartyWidget` _returnvalue)
  (`UserWidget.AddToViewport` _returnvalue -1))

(event `RemovePartyWidget`
  ;[1 1 1] 파티 리스트 위젯 생성 및 제거
  (`Widget.RemoveFromParent` (`self.PartyWidget`)))

(event `FieldTopMenu`
  (params (MenuSelect :type "/Game/Blueprints/Field/FieldTopMenuEnum Enum" :default "NewEnumerator0"))
  ;[1 1 1] 필드탑 메뉴 설정
  (`/Engine/EditorBlueprintResources/StandardMacros.IsValid` (`self.OtherPlayer`)
    (:`Is Valid`
      (switch `/Game/Blueprints/Field/FieldTopMenuEnum` MenuSelect
        (:`NewEnumerator0`
          ;[1 1 1] 파티 초대 위젯
          (`self.PartyInvateWidget` (`self.OtherPlayer`)))))
    (:`Is Not Valid`
      (if (`self.IsPartyInvate?`)
        (switch `/Game/Blueprints/Field/FieldTopMenuEnum` MenuSelect
          (:`NewEnumerator0`
            ;[1 1 1] 파티 탈퇴 위젯
            (if (`self.IsPartyOwner?`)
              (`self.PartyEscapeWidget` "파티장이 파티를 탈퇴 하면  \n파티가 소멸됩니다. \n그래도 탈퇴 하시겠습니까?")
              (else
                (`self.PartyEscapeWidget` "파티에서 탈퇴하시겠습니까?")))))))))

(fn `OnRep_PartyOwnerPawn`)

(fn `UserConstructionScript`)