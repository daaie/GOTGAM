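; TemplatePickup is a base field item, with mesh, image and texts set per instance through the construction script into its inventory struct.
; Its trigger toggles an in-range flag and a PickupText prompt widget for BP_FieldCharacter.
; It binds to the character's pickup event, but that handler is empty: the logic adding it to the HUD inventory and hiding it is disconnected.
; UseAction destroys the actor.
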(event `self.ReceiveBeginPlay`
  (bind _pickuptextreference (`self.PickupTextReference`))
  (bind _iteminfo (`self.ItemInfo`))
  (bind (_item _itemimage _pickuptext) (break `/Game/Blueprints/Field/InvertoryStruct` _iteminfo))
  ;[1 1 1] begin play
  (bind _returnvalue (`|CreateWidget` "/Game/UMG/Field/PickupText.PickupText_C"))
  (bind _output_get (set `self.PickupTextReference` _returnvalue))
  (`UserWidget.AddToViewport` _output_get 0)
  (`Widget.SetVisibility` _output_get "Hidden")
  (setmembers `/Game/Blueprints/Field/InvertoryStruct` :`StructRef` _iteminfo :`item` self)
  (set `/Game/UMG/Field/PickupText.PickupActor` _item _pickuptextreference)
  (set `/Game/UMG/Field/PickupText.PickupText` _pickuptext _pickuptextreference)
  (bind _asbp_field_character (cast `/Game/Blueprints/Field/BP_FieldCharacter` (`GameplayStatics.GetPlayerCharacter` 0)))
  (bind _output_get_2 (set `self.Character Ref` _asbp_field_character))
  (add `/Game/Blueprints/Field/BP_FieldCharacter.PickUpItem` _output_get_2 (delegate `PickupItem_이벤트_0`)))

(event `self.Trigger.OnComponentBeginOverlap`
  (params (OverlappedComponent :type "PrimitiveComponent Object Reference") (OtherActor :type "Actor Object Reference") (OtherComp :type "PrimitiveComponent Object Reference") (OtherBodyIndex :type Integer) (bFromSweep :type Boolean) (SweepResult :type "HitResult Structure (by ref)"))
  ;[1 1 1] 트리거 접근 스크립트
  (cast `/Game/Blueprints/Field/BP_FieldCharacter` OtherActor)
  (`Widget.SetVisibility` (`self.PickupTextReference`) "Visible")
  (set `self.IsInRange?` true))

(event `PickupItem_이벤트_0`
  ;[1 1 1] 아이템을 줍고 인벤토리에 넣은 다음 새로고침
)

(event `self.Trigger.OnComponentEndOverlap`
  (params (OverlappedComponent :type "PrimitiveComponent Object Reference") (OtherActor :type "Actor Object Reference") (OtherComp :type "PrimitiveComponent Object Reference") (OtherBodyIndex :type Integer))
  ;[1 1 1] 트리거 접근 스크립트
  (cast `/Game/Blueprints/Field/BP_FieldCharacter` OtherActor)
  (`Widget.SetVisibility` (`self.PickupTextReference`) "Hidden")
  (set `self.IsInRange?` false))

(event `/Game/Blueprints/Field/BP_Actioninterface.UseAction`
  ;[1 1 1] 아이템 사용하기
  (`self.K2_DestroyActor`))

(fn `UserConstructionScript`
  (setmembers `/Game/Blueprints/Field/InvertoryStruct` :`StructRef` (`self.ItemInfo`) :`item` self :`itemImage` (`self.CustomImage`) :`PickupText` (`self.CustomPickupText`) :`ActionText` (`self.CustomActionText`))
  (`StaticMeshComponent.SetStaticMesh` (`self.StaticMesh`) (`self.CustomStaticMesh`)))