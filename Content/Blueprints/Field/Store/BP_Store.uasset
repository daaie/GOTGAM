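; BP_Store is a field store actor that shows a shop UI while a player is inside its Sphere trigger.
; On overlap begin, only on non-authority instances, it creates a UMG_Store widget for the instigator's BP_FieldController, calls SetStoneMoney on it and adds it to the viewport.
; On overlap end, the same remote-side controller check removes the stored widget.
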(event `self.Sphere.OnComponentBeginOverlap`
  (params (OverlappedComponent :type "PrimitiveComponent Object Reference") (OtherActor :type "Actor Object Reference") (OtherComp :type "PrimitiveComponent Object Reference") (OtherBodyIndex :type Integer) (bFromSweep :type Boolean) (SweepResult :type "HitResult Structure (by ref)"))
  (`/Engine/EditorBlueprintResources/ActorMacros.Switch Has Authority`
    (:`Remote`
      (bind _asbp_field_controller (cast `/Game/Blueprints/Field/BP_FieldController` (`self.GetInstigatorController` OtherActor)))
      (`/Engine/EditorBlueprintResources/StandardMacros.IsValid` _asbp_field_controller
        (:`Is Valid`
          (bind _returnvalue (`|CreateWidget` "/Game/UMG/Field/UMG_Store.UMG_Store_C" _asbp_field_controller))
          (bind _output_get (set `self.StoreView` _returnvalue))
          (`/Game/UMG/Field/UMG_Store.SetStoneMoney` _output_get)
          (`UserWidget.AddToViewport` _output_get 0))))))

(event `self.Sphere.OnComponentEndOverlap`
  (params (OverlappedComponent :type "PrimitiveComponent Object Reference") (OtherActor :type "Actor Object Reference") (OtherComp :type "PrimitiveComponent Object Reference") (OtherBodyIndex :type Integer))
  (`/Engine/EditorBlueprintResources/ActorMacros.Switch Has Authority`
    (:`Remote`
      (bind _asbp_field_controller (cast `/Game/Blueprints/Field/BP_FieldController` (`self.GetInstigatorController` OtherActor)))
      (`/Engine/EditorBlueprintResources/StandardMacros.IsValid` _asbp_field_controller
        (:`Is Valid`
          (`Widget.RemoveFromParent` (`self.StoreView`)))))))

(fn `UserConstructionScript`)