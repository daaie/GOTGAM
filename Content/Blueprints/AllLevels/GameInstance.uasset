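; Game instance Blueprint that creates and shows the game's menus: login, character pick and creation, field and server.
; SaveGameCheck looks for the PlayerSettingsSave slot, opening the new character-pick menu if found, otherwise character creation.
; Show events mostly cache their widgets for reuse; Firld stores player count and server name, then opens a fresh server menu.
; Error-handling functions are empty stubs, and the save/load calls are unconnected.
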(event `SaveGameCheck`
  ;[1 1 1] Check  세이브 게임
  (bind _returnvalue (`GameplayStatics.DoesSaveGameExist` (`self.PlayerSettingsSave`)))
  (if _returnvalue
    (`self.Show NewPick Character Menu`)
    (set `self.CeratedSaveFile?` true)
    (else
      (`self.ShowCreateCharacterMenu`)
      (set `PlayerController.bShowMouseCursor` true (`GameplayStatics.GetPlayerController` 0)))))

(event `ShowPickCharacterMenu`
  ;[1 1 1] Show Pick Character Menu
  (`/Engine/EditorBlueprintResources/StandardMacros.IsValid` (`self.PickCharacteraMenuWB`)
    (:`Is Valid`
      _)
    (:`Is Not Valid`
      (bind _returnvalue (`|CreateWidget` "/Game/UMG/Main/UMG_PickCharacterMenu.UMG_PickCharacterMenu_C" (`GameplayStatics.GetPlayerController` 0)))
      (set `self.PickCharacteraMenuWB` _returnvalue)))
  (`UserWidget.AddToViewport` (`self.PickCharacteraMenuWB`) 0))

(event `ShowFieldMenu`
  ;[1 1 1] Show Field Menu
  (`/Engine/EditorBlueprintResources/StandardMacros.IsValid` (`self.FieldMenuWB`)
    (:`Is Not Valid`
      (bind _returnvalue (`|CreateWidget` "/Game/UMG/Field/UMG_FieldMenu.UMG_FieldMenu_C" (`GameplayStatics.GetPlayerController` 0)))
      (set `self.FieldMenuWB` _returnvalue)
      (`UserWidget.AddToViewport` (`self.FieldMenuWB`) 0))))

(event `Show Login Menu`
  (bind _returnvalue (`GameplayStatics.GetPlayerController` 0))
  ;[1 1 1] Show Login Menu
  (`/Engine/EditorBlueprintResources/StandardMacros.IsValid` (`self.Login Menu`)
    (:`Is Valid`
      _)
    (:`Is Not Valid`
      (bind _returnvalue_2 (`|CreateWidget` "/Game/UMG/Main/UMG_LoginMenu.UMG_LoginMenu_C" _returnvalue))
      (set `self.Login Menu` _returnvalue_2)))
  (`UserWidget.AddToViewport` (`self.Login Menu`) 0)
  (`WidgetBlueprintLibrary.SetInputMode_GameAndUIEx` _returnvalue _returnvalue_2)
  (set `PlayerController.bShowMouseCursor` true _returnvalue))

(event `Show NewPick Character Menu`
  ;[1 1 1] Show NewPick Character Menu
  (`/Engine/EditorBlueprintResources/StandardMacros.IsValid` (`self.NewPickCharacterMenu`)
    (:`Is Valid`
      _)
    (:`Is Not Valid`
      (bind _returnvalue (`|CreateWidget` "/Game/UMG/Main/UMG_NewPickCharacteraMenu.UMG_NewPickCharacteraMenu_C" (`GameplayStatics.GetPlayerController` 0)))
      (set `self.NewPickCharacterMenu` _returnvalue)))
  (`UserWidget.AddToViewport` (`self.NewPickCharacterMenu`) 0))

(event `Firld`
  (params (NumberOfPlayer :type Integer) (`EnableLan?` :type Boolean) (ServerName :type Text))
  ;[1 1 1] 라우터랑 Lobby 셋팅
  (set `self.MaxPlayer` NumberOfPlayer)
  (set `self.ServerName` ServerName)
  (bind _returnvalue (`|CreateWidget` "/Game/UMG/Main/Server/UMG_ServerMenu.UMG_ServerMenu_C"))
  (`UserWidget.AddToViewport` _returnvalue 0))

(event `ShowCreateCharacterMenu`
  ;[1 1 1] Show Create Character Menu
  (`/Engine/EditorBlueprintResources/StandardMacros.IsValid` (`self.ShowCreateChatacterMenu`)
    (:`Is Valid`
      _)
    (:`Is Not Valid`
      (bind _returnvalue (`|CreateWidget` "/Game/UMG/Main/UMG_CreateCharacterMenu.UMG_CreateCharacterMenu_C" (`GameplayStatics.GetPlayerController` 0)))
      (set `self.ShowCreateChatacterMenu` _returnvalue)))
  (`UserWidget.AddToViewport` (`self.ShowCreateChatacterMenu`) 0))

(fn `NetErrorToString`
  (params (FailureType :type "ENetworkFailure Enum" :default "NetDriverAlreadyExists"))
  (returns (OutString :type String))
  (return ""))

(fn `TravelErrorToString`
  (params (FailureType :type "ETravelFailure Enum" :default "NoLevel"))
  (returns (OutSring :type String))
  (return ""))