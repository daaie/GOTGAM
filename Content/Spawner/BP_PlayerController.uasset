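; Player controller blueprint that runs test actions for four slot-based combat commands: attack, defend, run and capture.
; Each acts on the FirstPersonGameMode PlayerS actor at TestSlot, then increments the slot.
; Attack uses timeline lerps to move the actor toward TestAI_Enemy target locations and back.
; Run lifts the actor by timeline and destroys it, while defend and capture are placeholders that spawn an explosion and print.
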(event `testNext`
  ;[1 1 1] 테스트용: 다음 슬롯 지정
  (`/Engine/EditorBlueprintResources/StandardMacros.IncrementInt` (`self.testSlot`)))

(event `AttackActFunc`
  (bind _testslot (`self.testSlot`))
  ;[1 1 1] 1. 공격버튼
  (bind _asfirst_person_game_mode (cast `/Game/FirstPersonBP/Blueprints/FirstPersonGameMode` (`GameplayStatics.GetGameMode`)))
  (bind _players (`/Game/FirstPersonBP/Blueprints/FirstPersonGameMode.PlayerS` _asfirst_person_game_mode))
  (set `self.StartLocation` (`self.K2_GetActorLocation` (`|GetArrayItem` _players _testslot)))
  (bind (_direction _move) (`Timeline|타임라인_0` :!via `PlayFromStart`)
    (:`Update`
      (bind _outactors (`GameplayStatics.GetAllActorsOfClass` "/Game/Spawner/TestAI_Enemy.TestAI_Enemy_C"))
      (for _array_element _outactors
        (bind _output (`|GetArrayItem` _players _testslot))
        (bind _rootcomponent (`Actor.RootComponent` _output))
        (`SceneComponent.K2_SetWorldLocation` _rootcomponent (`KismetMathLibrary.VLerp` (`self.StartLocation`) (`/Game/Spawner/TestAI_Enemy.TargetLoc` _array_element) _move) true true)))
    (:`Finished`
      (bind (_direction_2 _move_2) (`Timeline|타임라인_1` :!via `PlayFromStart`)
        (:`Update`
          (`SceneComponent.K2_SetWorldLocation` _rootcomponent (`KismetMathLibrary.VLerp` (`self.K2_GetActorLocation` _output) (`self.StartLocation`) _move_2) false true))
        (:`Finished`
          (`self.testNext`))))))

(event `RunActFunc`
  (bind _testslot (`self.testSlot`))
  ;[1 1 1] 3. 도망버튼
  (bind _asfirst_person_game_mode (cast `/Game/FirstPersonBP/Blueprints/FirstPersonGameMode` (`GameplayStatics.GetGameMode`)))
  (bind (_direction _move) (`Timeline|타임라인_2` :!via `PlayFromStart`)
    (:`Update`
      (bind _output (`|GetArrayItem` (`/Game/FirstPersonBP/Blueprints/FirstPersonGameMode.PlayerS` _asfirst_person_game_mode) _testslot))
      (bind _returnvalue (`self.K2_GetActorLocation` _output))
      (`SceneComponent.K2_SetWorldLocation` (`Actor.RootComponent` _output) (`KismetMathLibrary.VLerp` _returnvalue (+ _returnvalue (0.0 0.0 100.0)) _move) true false))
    (:`Finished`
      (`self.K2_DestroyActor` _output)
      (`KismetSystemLibrary.PrintString` (`KismetStringLibrary.Concat_StrStr` "Player" (`KismetStringLibrary.Conv_IntToString` _testslot) ": Run Success!") true true (struct :`G` 0.66 :`B` 1.0 :`A` 1.0) 5.0)
      (`self.testNext`))))

(event `CaptureActFunc`
  ;[1 1 1] 4. 포획 버튼
  (bind _asfirst_person_game_mode (cast `/Game/FirstPersonBP/Blueprints/FirstPersonGameMode` (`GameplayStatics.GetGameMode`)))
  (`GameplayStatics.SpawnEmitterAtLocation` "/Game/StarterContent/Particles/P_Explosion.P_Explosion" (`self.K2_GetActorLocation` (`|GetArrayItem` (`/Game/FirstPersonBP/Blueprints/FirstPersonGameMode.PlayerS` _asfirst_person_game_mode) (`self.testSlot`))))
  (`KismetSystemLibrary.PrintString` "4. Capture Button is clicked")
  (`self.testNext`))

(event `DepenceActFunc`
  ;[1 1 1] 2. 방어버튼
  (bind _asfirst_person_game_mode (cast `/Game/FirstPersonBP/Blueprints/FirstPersonGameMode` (`GameplayStatics.GetGameMode`)))
  (`GameplayStatics.SpawnEmitterAtLocation` "/Game/StarterContent/Particles/P_Explosion.P_Explosion" (`self.K2_GetActorLocation` (`|GetArrayItem` (`/Game/FirstPersonBP/Blueprints/FirstPersonGameMode.PlayerS` _asfirst_person_game_mode) (`self.testSlot`))))
  (`KismetSystemLibrary.PrintString` "2. Depence Button is clicked")
  (`self.testNext`))

(fn `UserConstructionScript`)