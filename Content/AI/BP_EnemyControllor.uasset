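; BP_EnemyControllor is the enemy AI controller, which starts the enemy blackboard and behavior tree on BeginPlay.
; Every Tick it checks the IsTurnOver flag, which nothing in this graph sets.
; While that flag is true, it rewrites the blackboard keys each frame to enable attack and defence and disable run.
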(event `self.ReceiveBeginPlay`
  (`self.UseBlackboard` "/Game/AI/BTB_Enemy.BTB_Enemy")
  (`self.RunBehaviorTree` "/Game/AI/BTT_Enemy.BTT_Enemy"))

(event `self.ReceiveTick`
  (params (DeltaSeconds :type "Float (single-precision)"))
  (if (`self.IsTurnOver?`)
    (`BlackboardComponent.SetValueAsBool` (`AIBlueprintHelperLibrary.GetBlackboard` null) "IsAttack?" true)
    (`BlackboardComponent.SetValueAsBool` (`AIBlueprintHelperLibrary.GetBlackboard` null) "IsDefence?" true)
    (`BlackboardComponent.SetValueAsBool` (`AIBlueprintHelperLibrary.GetBlackboard` null) "IsRun?" false)))

(fn `UserConstructionScript`)